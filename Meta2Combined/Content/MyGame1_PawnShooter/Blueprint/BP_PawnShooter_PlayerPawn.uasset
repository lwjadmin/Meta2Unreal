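; BP_PawnShooter_PlayerPawn is the player pawn for a shooter, with free movement, mouse-look style controls and click-to-shoot.
; Axis inputs offset the pawn along camera forward and right vectors without sweeping, and feed controller yaw and pitch, with yaw input also printed.
; Left click line-traces from the pawn along camera forward with debug drawing, destroying any hit actor that implements BPI_PawnShooter_Target.
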(event Input|AxisEvents|InputAxisMoveForward
  (params (AxisValue :type Float%20%28single-precision%29))
  (Transformation|AddActorLocalOffset (* (Transformation|GetActorForwardVector (Game|GetPlayerCameraManager 0)) (* AxisValue (Variables|Default|GetMoveSpeed))) false false))

(event Input|AxisEvents|InputAxisMoveRight
  (params (AxisValue :type Float%20%28single-precision%29))
  (Transformation|AddActorLocalOffset (* (Transformation|GetActorRightVector (Game|GetPlayerCameraManager 0)) (* AxisValue (Variables|Default|GetMoveSpeed))) false false))

(event Input|AxisEvents|InputAxisLookUp
  (params (AxisValue :type Float%20%28single-precision%29))
  (Pawn|Input|AddControllerPitchInput AxisValue))

(event Input|AxisEvents|InputAxisTurn
  (params (AxisValue :type Float%20%28single-precision%29))
  (Development|PrintString (Utilities|String|ToString(Float) AxisValue))
  (Pawn|Input|AddControllerYawInput AxisValue))

(event Input|MouseEvents|LeftMouseButton
  (params (Key :type Key%20Structure :default "None"))
  (bind _returnvalue (Transformation|GetActorLocation))
  (:Pressed
    (bind (_outhit _returnvalue_2) (Collision|LineTraceByChannel _returnvalue (+ _returnvalue (* (Math|Vector|GetForwardVector (Transformation|GetActorRotation (Game|GetPlayerCameraManager 0))) 10000)) "TraceTypeQuery1" false 0 "ForDuration"))
    (if (and _returnvalue_2 (Utilities|DoesObjectImplementInterface (.HitActor (Collision|BreakHitResult _outhit)) "/Game/MyGame1_PawnShooter/Blueprint/BPI_PawnShooter_Target.BPI_PawnShooter_Target_C"))
      (Actor|DestroyActor (.HitActor (Collision|BreakHitResult _outhit))))))

(fn ConstructionScript)