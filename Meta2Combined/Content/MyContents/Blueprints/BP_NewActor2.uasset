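; BP_NewActor2 is a sphere actor, apparently an event dispatcher test, that destroys "PAN"-tagged actors it hits with an explosion effect and sound.
; BeginPlay binds three print handlers to one dispatcher and unbinds the third, so each hit prints from the remaining two.
; EndPlay plays the same explosion at the sphere's own location.
; SetPhysics and Print are empty, and the simulate-physics call is unconnected.
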(event OnComponentHit(Sphere)
  (params (HitComponent :type Primitive%20Component%20Object%20Reference) (OtherActor :type Actor%20Object%20Reference) (OtherComp :type Primitive%20Component%20Object%20Reference) (NormalImpulse :type Vector :default "0, 0, 0") (Hit :type Hit%20Result%20Structure%20%28by%20ref%29))
  (Default|CallNewEventDispatcher)
  (if (Actor|ActorHasTag OtherActor "PAN")
    (Transformation|AddActorLocalRotation "0, 0, 0" false false)
    (Effects|SpawnEmitteratLocation "/Game/StarterContent/Particles/P_Explosion.P_Explosion" (Transformation|GetActorLocation OtherActor))
    (Audio|PlaySound2D "/Game/StarterContent/Audio/Explosion01.Explosion01" 1.0 1.0 0.0 0 0)
    (Actor|DestroyActor OtherActor)))

(event Custom|NewEventDispatcher_Event_0
  (Development|PrintString "1111"))

(event Custom|NewEventDispatcher_Event_1
  (Development|PrintString "2222"))

(event Custom|NewEventDispatcher_Event_2
  (Development|PrintString "3333"))

(event Custom|SetPhysics)

(event EventBeginPlay
  (EventDispatchers|AssignNewEventDispatcher (delegate Custom|NewEventDispatcher_Event_0))
  (EventDispatchers|AssignNewEventDispatcher (delegate Custom|NewEventDispatcher_Event_1))
  (EventDispatchers|AssignNewEventDispatcher (delegate Custom|NewEventDispatcher_Event_2))
  (EventDispatchers|UnbindEventfromNewEventDispatcher (delegate Custom|NewEventDispatcher_Event_2)))

(event EventEndPlay
  (params (EndPlayReason :type EEndPlayReason%20Enum :default "Destroyed"))
  ;[1 1 1] 삭제될 예정일때 호출
  (Effects|SpawnEmitteratLocation "/Game/StarterContent/Particles/P_Explosion.P_Explosion" (Transformation|GetActorLocation))
  (Audio|PlaySound2D "/Game/StarterContent/Audio/Explosion01.Explosion01" 1.0 1.0 0.0 0 0))

(event EventPrint)

(fn ConstructionScript)