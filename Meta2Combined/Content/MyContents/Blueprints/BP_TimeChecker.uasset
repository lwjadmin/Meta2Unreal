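; BP_TimeChecker is a hold-timing mini-game actor that judges how long the player holds the left mouse button.
; It enables player input on BeginPlay; pressing opens a gate so Tick accumulates elapsed time and prints an in-game status.
; Releasing closes the gate, prints success or failure depending on whether the time falls in a four-to-five-second window, then resets the timer.
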(event EventTick
  (params (DeltaSeconds :type Float%20%28single-precision%29))
  (Utilities|FlowControl|Gate true
    (:Exit
      (bind _output_get (Variables|Default|SetTime (+ (Variables|Default|GetTime) DeltaSeconds)))
      (Development|PrintString "게임중" true true "(R=0.000000,G=0.660000,B=1.000000,A=1.000000)" 0.0))))

(event EventBeginPlay
  (Input|EnableInput (Game|GetPlayerController 0)))

(event Input|MouseEvents|LeftMouseButton
  (params (Key :type Key%20Structure :default "None"))
  (:Pressed
    (Utilities|FlowControl|Gate true) ; enters at Open
  )
  (:Released
    (Utilities|FlowControl|Sequence
      (:then_0
        (Utilities|FlowControl|Gate true) ; enters at Close
      )
      (:then_1
        (if (and (>= (Variables|Default|GetTime) 4.0) (<= (Variables|Default|GetTime) 5.0))
          (Development|PrintString (Utilities|String|Append (Utilities|String|ToString(Float) (Variables|Default|GetTime)) "초, 성공!"))
          (else
            (Development|PrintString (Utilities|String|Append (Utilities|String|ToString(Float) (Variables|Default|GetTime)) "초, 실패!")))))
      (:then_2
        (Variables|Default|SetTime 0.0)))))

(fn ConstructionScript)