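; BP_CustomSpotLight1 is a spotlight actor that stays hidden until switched on and rotates in steps.
; The spotlight is hidden at construction and BeginPlay, and the EvtLightson and EvtLightsOff events toggle its visibility.
; Tick accumulates time and applies a fixed world rotation roughly every tenth of a second, whether the light is visible or not.
; The EvtLightsRotate event is empty.
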(event EventBeginPlay
  (Rendering|SetVisibility (Variables|Default|GetSpotLight) false false))

(event Collision|EventActorBeginOverlap
  (params (OtherActor :type Actor%20Object%20Reference)))

(event EventTick
  (params (DeltaSeconds :type Float%20%28single-precision%29))
  (bind _output_get (Variables|Default|SetInterval (+ (Variables|Default|GetInterval) DeltaSeconds)))
  (if (>= _output_get 0.1)
    (Transformation|AddWorldRotation (Variables|Default|GetSpotLight) "0,15.000000, 0" false false)
    (Variables|Default|SetInterval 0.0)))

(event EventEvtLightson
  (Rendering|SetVisibility (Variables|Default|GetSpotLight) true false))

(event EventEvtLightsOff
  (Rendering|SetVisibility (Variables|Default|GetSpotLight) false false))

(event EventEvtLightsRotate)

(fn ConstructionScript
  (Rendering|SetVisibility (Variables|Default|GetSpotLight) false false))