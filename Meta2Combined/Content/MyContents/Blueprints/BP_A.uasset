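; BP_A is a simple test actor that displays its own name on a TextRender component.
; On BeginPlay it sets the text to its display name.
; A custom Print event prints the name with a hello greeting to the screen and shows the same message on the text component.
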(event EventBeginPlay
  (Rendering|Components|TextRender|SetText (Variables|Default|GetTextRender) (Utilities|Text|ToText(String) (Utilities|GetDisplayName self))))

(event EventPrint
  (bind _self self)
  (bind _returnvalue (Utilities|GetDisplayName _self))
  (bind _returnvalue_2 (Utilities|String|Append _returnvalue " : Hello!"))
  (Development|PrintString _returnvalue_2)
  (Rendering|Components|TextRender|SetText (Variables|Default|GetTextRender) (Utilities|Text|ToText(String) _returnvalue_2)))

(fn ConstructionScript)