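; BP_CleanActor is an actor that tracks and prints its elapsed running time on screen as minutes and seconds.
; Each Tick adds DeltaSeconds to ElapsedTime, derives minutes by division and seconds by modulo, and prints the combined string.
; The IntStrZeroZero helper floors each value and pads it with a leading zero below ten.
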(event EventTick
  (params (DeltaSeconds :type Float%20%28single-precision%29))
  (bind _output_get (Variables|Default|SetElapsedTime (+ DeltaSeconds (Variables|Default|GetElapsedTime))))
  (bind _strout (CallFunction|IntStrZeroZero (/ _output_get 6e+01)))
  (bind _strout_2 (CallFunction|IntStrZeroZero (Math|Float|%(Float) _output_get 6e+01)))
  (Development|PrintString (Utilities|String|Append "Elapsed Time : " _strout "Minutes, " _strout_2 "Seconds")))

(fn ConstructionScript)

(fn IntStrZeroZero
  (params (fval :type Float%20%28single-precision%29))
  (bind _returnvalue (Math|Float|Floor fval))
  (bind _returnvalue_2 (Utilities|String|ToString(Integer) _returnvalue))
  (if (< _returnvalue 10)
    (return (Utilities|String|Append "0" _returnvalue_2))
    (else
      (return _returnvalue_2))))