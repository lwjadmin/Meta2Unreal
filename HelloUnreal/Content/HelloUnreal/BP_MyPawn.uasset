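; BP_MyPawn is a free-flying player pawn, apparently for input testing, that moves and looks around through legacy input axis and action mappings.
; Movement offsets the actor without sweep along the camera manager's forward and right vectors, scaled by MoveSpeed but not delta time; look axes feed controller pitch and yaw.
; Speed actions step MoveSpeed within a clamped range and print it.
; An elapsed-time printer and older speed-step logic remain unconnected, and several debug prints have output disabled.
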(event EventBeginPlay
  (Development|PrintString (Utilities|GetDisplayName self) false false "(R=0.000000,G=0.660000,B=1.000000,A=1.000000)" 6e+01))

(event EventTick
  (params (DeltaSeconds :type Float%20%28single-precision%29)))

(event Input|ActionEvents|InputActionTestKey
  (params (Key :type Key%20Structure :default "None"))
  (bind _returnvalue (Class|KismetInputLibrary|KeyGetDisplayName Key))
  (bind _returnvalue_2 (Utilities|String|ToString(Text) _returnvalue))
  (:Pressed
    (Development|PrintString (Utilities|String|Append _returnvalue_2 " Key Pressed") false false))
  (:Released
    (Development|PrintString (Utilities|String|Append _returnvalue_2 " Key Released") false false)))

(event Input|ActionEvents|InputActionSpeedUp
  (params (Key :type Key%20Structure :default "None"))
  (:Pressed
    (bind _output_get (Variables|Default|SetMoveSpeed (Math|Float|Clamp(Float) (+ (Variables|Default|GetMoveSpeed) 1e+01) 1e+01 1e+02)))
    (Development|PrintString (Utilities|String|Append "MoveSpd : " (Utilities|String|ToString(Float) _output_get)))))

(event Input|ActionEvents|InputActionSpeedDown
  (params (Key :type Key%20Structure :default "None"))
  (:Pressed
    (bind _output_get (Variables|Default|SetMoveSpeed (Math|Float|Clamp(Float) (- (Variables|Default|GetMoveSpeed) 1e+01) 1e+01 1e+02)))
    (Development|PrintString (Utilities|String|Append "MoveSpd : " (Utilities|String|ToString(Float) _output_get)))))

(event Input|ActionEvents|InputActionSpeedUp
  (params (Key :type Key%20Structure :default "None")))

(event Input|ActionEvents|InputActionSpeedDown
  (params (Key :type Key%20Structure :default "None")))

(event Input|AxisEvents|InputAxisAxisTest
  (params (AxisValue :type Float%20%28single-precision%29))
  (Development|PrintString (Utilities|String|Append "Axis Value : " (Utilities|String|ToString(Float) AxisValue)) false false))

(event Input|AxisEvents|InputAxisMoveForward
  (params (AxisValue :type Float%20%28single-precision%29))
  (Transformation|AddActorWorldOffset (* (Transformation|GetActorForwardVector (Game|GetPlayerCameraManager 0)) (* AxisValue (Variables|Default|GetMoveSpeed)))))

(event Input|AxisEvents|InputAxisMoveRight
  (params (AxisValue :type Float%20%28single-precision%29))
  (Transformation|AddActorWorldOffset (* (Transformation|GetActorRightVector (Game|GetPlayerCameraManager 0)) (* AxisValue (Variables|Default|GetMoveSpeed)))))

(event Input|AxisEvents|InputAxisLookUp
  (params (AxisValue :type Float%20%28single-precision%29))
  (Pawn|Input|AddControllerPitchInput AxisValue))

(event Input|AxisEvents|InputAxisLookRight
  (params (AxisValue :type Float%20%28single-precision%29))
  (Pawn|Input|AddControllerYawInput AxisValue))

(fn ConstructionScript)

(fn InttoStrZeroZero
  (params (fval :type Float%20%28single-precision%29))
  (bind _returnvalue (Math|Float|Floor fval))
  (bind _returnvalue_2 (Utilities|String|ToString(Integer) _returnvalue))
  (if (< _returnvalue 10)
    (return (Utilities|String|Append "0" _returnvalue_2))
    (else
      (return _returnvalue_2))))

(fn PrintTime
  (params (DeltaSeconds :type Float%20%28single-precision%29))
  (bind _output_get (Variables|Default|SetTotalDeltaSeconds (+ DeltaSeconds (Variables|Default|GetTotalDeltaSeconds))))
  (if (Utilities|Enum|NotEqual(Enum) (Utilities|String|Append "result : " (Custom1|InttoStrZeroZero (/ _output_get 6e+01)) "min " (Custom1|InttoStrZeroZero (Math|Float|%(Float) _output_get 6e+01)) "sec") (Variables|Default|GetnextString))
    (Development|PrintString (Utilities|String|Append "result : " (Custom1|InttoStrZeroZero (/ _output_get 6e+01)) "min " (Custom1|InttoStrZeroZero (Math|Float|%(Float) _output_get 6e+01)) "sec") true true "(R=0.000000,G=0.660000,B=1.000000,A=1.000000)" 6e+01)
    (Variables|Default|SetnextString (Utilities|String|Append "result : " (Custom1|InttoStrZeroZero (/ _output_get 6e+01)) "min " (Custom1|InttoStrZeroZero (Math|Float|%(Float) _output_get 6e+01)) "sec"))))