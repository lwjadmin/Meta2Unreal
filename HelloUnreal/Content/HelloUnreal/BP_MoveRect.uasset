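; BP_MoveRect is an actor that moves its static mesh around a square loop in the local XZ plane.
; BeginPlay starts a looping timer that calls UpdateMove at a short fixed interval instead of using Tick.
; UpdateMove switches on the MoveType direction state, nudging the mesh by a fixed step and advancing to the next direction once it passes that side's limit.
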(event EventBeginPlay
  (Utilities|Time|SetTimerbyFunctionName 0 "UpdateMove" 0.01 true))

(fn ConstructionScript)

(fn UpdateMove
  (bind _staticmesh (Variables|Default|GetStaticMesh))
  (switch Utilities|FlowControl|Switch|SwitchonEnum_MoveType (Variables|Default|GetMoveType)
    (:NewEnumerator0
      (Transformation|AddRelativeLocation _staticmesh "5.000000, 0, 0" false false)
      (if (> (.x (Variables|/Script/Engine.SceneComponent|GetRelativeLocation (Variables|Default|GetStaticMesh))) 3e+02)
        (Variables|Default|SetMoveType "NewEnumerator1")))
    (:NewEnumerator1
      (Transformation|AddRelativeLocation _staticmesh "0.000000,0.000000,5.000000" false false)
      (if (> (.z (Variables|/Script/Engine.SceneComponent|GetRelativeLocation (Variables|Default|GetStaticMesh))) 3e+02)
        (Variables|Default|SetMoveType "NewEnumerator2")))
    (:NewEnumerator2
      (Transformation|AddRelativeLocation _staticmesh "-5.000000, 0, 0" false false)
      (if (< (.x (Variables|/Script/Engine.SceneComponent|GetRelativeLocation (Variables|Default|GetStaticMesh))) 0.0)
        (Variables|Default|SetMoveType "NewEnumerator3")))
    (:NewEnumerator3
      (Transformation|AddRelativeLocation _staticmesh "0.000000, 0,-5.000000" false false)
      (if (< (.z (Variables|/Script/Engine.SceneComponent|GetRelativeLocation (Variables|Default|GetStaticMesh))) 0.0)
        (Variables|Default|SetMoveType "NewEnumerator0")))))