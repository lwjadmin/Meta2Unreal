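; Third-person shooter player Blueprint handling movement, health, stamina, aiming, ammo and HUD.
; Input flags set walk speed; sprinting and jumping drain stamina, and aiming switches to controller yaw with a timeline FOV zoom.
; While Fire and Aim are held, a Tick-fed Gate and Delay throttle camera-based hitscan shots.
; Damage triggers camera shake and timeline-blended physical hit reactions from spine_01; death disables input and ragdolls the mesh.
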(event Custom|EventGetAmmunition
  (Variables|Default|SetMaxAmmoCount (+ (Variables|Default|GetMaxAmmoCount) (Variables|Default|GetAmmoMagazineSize)))
  (Audio|PlaySound2D 0 1.0 1.0 0.0 0 0))

(event Custom|ShowGUI
  ;[1 1 1] Default Loading
  (Utilities|IsValid (Variables|Default|GetRefGUIWidget)
    (:Is%20Not%20Valid
      (bind _returnvalue (UserInterface|CreateWidget "/Game/MyContents/Player/UMG_PlayerUI.UMG_PlayerUI_C" (Game|GetPlayerController 0)))
      (bind _output_get (Variables|Default|SetRefGUIWidget _returnvalue))
      (UserInterface|Viewport|AddtoViewport _output_get 0))))

(event Custom|SetDefaultMode
  (bind _self self)
  (bind _springarm (Variables|Default|GetSpringArm))
  (bind _charactermovement (Variables|Character|GetCharacterMovement))
  ;[1 1 1] Default Loading
  (Variables|Default|SetTags _self (Utilities|Array|MakeArray "Player"))
  (Variables|Default|SetbUseControllerRotationYaw _self false)
  (Variables|/Script/Engine.SpringArmComponent|SetbEnableCameraLag _springarm true)
  (Variables|/Script/Engine.SpringArmComponent|SetbUsePawnControlRotation _springarm true)
  (Variables|/Script/Engine.CharacterMovementComponent|SetbOrientRotationToMovement _charactermovement true)
  (Variables|/Script/Engine.CharacterMovementComponent|SetbUseControllerDesiredRotation _charactermovement true))

(event EventBeginPlay
  ;[1 1 1] Default Loading
  (CallFunction|SetDefaultMode)
  (CallFunction|ShowGUI))

(event Game|Damage|EventAnyDamage
  (params (Damage :type Float%20%28single-precision%29) (DamageType :type Damage%20Type%20Object%20Reference) (InstigatedBy :type Controller%20Object%20Reference) (DamageCauser :type Actor%20Object%20Reference))
  (bind _returnvalue (Utilities|Name|MakeLiteralName "spine_01"))
  (bind _mesh (Variables|Character|GetMesh))
  ;[1 1 1] Damaged & Die
  (if (not (Variables|Default|GetbIsDead))
    (bind _output_get (Variables|Default|SetbIsDead (<= (- (Variables|Default|GetCurHP) Damage) 0.0)))
    (if _output_get
      (Variables|Default|SetCurHP 0.0)
      (Utilities|FlowControl|Sequence
        (:then_0
          (bind _blendweight (Timeline|ChangeBlendWeight Stop)
            (:Update
              (Class|SkeletalMeshComponent|SetAllBodiesBelowPhysicsBlendWeight _mesh _returnvalue _blendweight false true))
            (:Finished
              (Class|SkeletalMeshComponent|SetAllBodiesBelowSimulatePhysics _mesh _returnvalue false true))))
        (:then_1
          (Class|SkeletalMeshComponent|SetAllBodiesBelowPhysicsBlendWeight _mesh _returnvalue 0.0 false true)
          (Input|DisableInput (Game|GetPlayerController 0))
          (Physics|SetSimulatePhysics (Variables|Character|GetMesh) true)
          (Collision|SetCollisionEnabled (Variables|Collision|GetCapsuleComponent) "NoCollision")
          (Pawn|Components|CharacterMovement|DisableMovement (Variables|Character|GetCharacterMovement))
          (Audio|PlaySound2D 0 1.0 1.0 0.0 0 0)))
      (else
        (Variables|Default|SetCurHP (- (Variables|Default|GetCurHP) Damage))
        (Utilities|FlowControl|Sequence
          (:then_0
            (CameraShakes|StartCameraShake (Game|GetPlayerCameraManager 0) "/Game/MyContents/Player/BP_Player_Damaged_CamShake.BP_Player_Damaged_CamShake_C" 1.0 "CameraLocal" "0, 0, 0")
            (Audio|PlaySound2D 0 1.0 1.0 0.0 0 0)
            (Class|SkeletalMeshComponent|SetAllBodiesBelowSimulatePhysics _mesh _returnvalue true true)
            (Timeline|ChangeBlendWeight PlayFromStart)))))))

(event EventTick
  (params (DeltaSeconds :type Float%20%28single-precision%29))
  (bind _maxstamina (Variables|Default|GetMaxStamina))
  (bind _curammocount (Variables|Default|GetCurAmmoCount))
  (Utilities|FlowControl|Sequence
    (:then_0
      (if (and (Variables|Default|GetbSprintPressed) (not (Variables|Default|GetbIsDead)))
        (Variables|Default|SetCurStamina (Math|Float|Clamp(Float) (- (Variables|Default|GetCurStamina) (* DeltaSeconds 2e+01)) 0.0 _maxstamina))
        (else
          (Variables|Default|SetCurStamina (Math|Float|Clamp(Float) (+ (Variables|Default|GetCurStamina) (* DeltaSeconds 1e+01)) 0.0 _maxstamina))))
      (CallFunction|SetCharacterWalkSpeed))
    (:then_1
      (Utilities|FlowControl|Gate true
        (:Exit
          (if (Variables|Default|GetbAimPressed)
            (Utilities|FlowControl|Delay 0.1)
            (CallFunction|Fire 100000 _curammocount)
            (if (> _curammocount 0)
              (Math|Integer|DecrementInt _curammocount))))))))

(event Input|ActionEvents|InputActionSprint
  (params (Key :type Key%20Structure :default "None"))
  (:Pressed
    (if (> (/ (Variables|Default|GetCurStamina) (Variables|Default|GetMaxStamina)) 0.3)
      (Variables|Default|SetbSprintPressed true)
      (CallFunction|SetCharacterWalkSpeed :!label _label)))
  (:Released
    (Variables|Default|SetbSprintPressed false)
    (goto _label)))

(event Input|ActionEvents|InputActionCrouch
  (params (Key :type Key%20Structure :default "None"))
  (:Pressed
    (Variables|Default|SetbCrouchPressed (not (Variables|Default|GetbCrouchPressed)))
    (CallFunction|SetCharacterWalkSpeed)))

(event Input|ActionEvents|InputActionWalk
  (params (Key :type Key%20Structure :default "None"))
  (:Pressed
    (Variables|Default|SetbWalkPressed true)
    (CallFunction|SetCharacterWalkSpeed :!label _label))
  (:Released
    (Variables|Default|SetbWalkPressed false)
    (goto _label)))

(event Input|ActionEvents|InputActionFire
  (params (Key :type Key%20Structure :default "None"))
  (bind _curammocount (Variables|Default|GetCurAmmoCount))
  (:Pressed
    (Utilities|FlowControl|Gate true) ; enters at Open
  )
  (:Released
    (Utilities|FlowControl|Gate true) ; enters at Close
  ))

(event Input|ActionEvents|InputActionReload
  (params (Key :type Key%20Structure :default "None"))
  (bind _ammomagazinesize (Variables|Default|GetAmmoMagazineSize))
  (:Pressed
    (if (< (Variables|Default|GetCurAmmoCount) (Variables|Default|GetAmmoMagazineSize))
      (if (>= (Variables|Default|GetMaxAmmoCount) (Variables|Default|GetAmmoMagazineSize))
        (Variables|Default|SetMaxAmmoCount (- (+ (Variables|Default|GetMaxAmmoCount) (Variables|Default|GetCurAmmoCount)) _ammomagazinesize) :!label _label)
        (Variables|Default|SetCurAmmoCount _ammomagazinesize)
        (Audio|PlaySound2D 0 1.0 1.0 0.0 0 0)
        (Variables|Default|SetbReloadPressed true)
        (elif (>= (+ (Variables|Default|GetCurAmmoCount) (Variables|Default|GetMaxAmmoCount)) (Variables|Default|GetAmmoMagazineSize))
          (goto _label)
          (elif (> (Variables|Default|GetMaxAmmoCount) 0)
            ;[1 1 1] Last One!
            (Variables|Default|SetCurAmmoCount (+ (Variables|Default|GetMaxAmmoCount) (Variables|Default|GetCurAmmoCount)))
            (Variables|Default|SetMaxAmmoCount 0)))))))

(event Input|ActionEvents|InputActionJump
  (params (Key :type Key%20Structure :default "None"))
  (:Pressed
    (if (not (Variables|Default|GetbJumpPressed))
      (Variables|Default|SetCurStamina (* (Variables|Default|GetCurStamina) 0.9))
      (Character|Jump)
      (Variables|Default|SetbJumpPressed true)))
  (:Released
    (Character|StopJumping)))

(event Input|ActionEvents|InputActionAim
  (params (Key :type Key%20Structure :default "None"))
  (bind _charactermovement (Variables|Character|GetCharacterMovement))
  (:Pressed
    (if (not (or (Variables|Default|GetbSprintPressed) (Variables|Default|GetbJumpPressed)))
      (Variables|Default|SetbAimPressed true)
      (CallFunction|SetCharacterWalkSpeed)
      (Utilities|IsValid (Variables|Default|GetRefGUIAimWidget)
        (:Is%20Valid
          _)
        (:Is%20Not%20Valid
          (bind _returnvalue (UserInterface|CreateWidget "/Game/MyContents/Player/UMG_PlayerAimUI.UMG_PlayerAimUI_C"))
          (bind _output_get (Variables|Default|SetRefGUIAimWidget _returnvalue))))
      (UserInterface|Viewport|AddtoViewport _output_get 0)
      (Utilities|FlowControl|Sequence
        (:then_0
          (Variables|/Script/Engine.CharacterMovementComponent|SetbUseControllerDesiredRotation _charactermovement false)
          (Variables|/Script/Engine.CharacterMovementComponent|SetbOrientRotationToMovement _charactermovement false)
          (Variables|Default|SetbUseControllerRotationYaw true))
        (:then_1
          (bind _fieldofview (Timeline|타임라인_0 Play)
            (:Update
              (Camera|SetFieldOfView (Variables|Default|GetCamera) _fieldofview)))))))
  (:Released
    (Variables|Default|SetbAimPressed false)
    (CallFunction|SetCharacterWalkSpeed)
    (Utilities|IsValid (Variables|Default|GetRefGUIAimWidget)
      (:Is%20Valid
        (Widget|RemovefromParent _output_get)
        (Utilities|FlowControl|Sequence
          (:then_0
            (Variables|/Script/Engine.CharacterMovementComponent|SetbUseControllerDesiredRotation _charactermovement true)
            (Variables|/Script/Engine.CharacterMovementComponent|SetbOrientRotationToMovement _charactermovement true)
            (Variables|Default|SetbUseControllerRotationYaw false))
          (:then_1
            (Timeline|타임라인_0 Reverse)))))))

(event Input|AxisEvents|InputAxisLookUp
  (params (AxisValue :type Float%20%28single-precision%29))
  (Pawn|Input|AddControllerPitchInput AxisValue))

(event Input|AxisEvents|InputAxisTurn
  (params (AxisValue :type Float%20%28single-precision%29))
  (Pawn|Input|AddControllerYawInput AxisValue))

(event Input|AxisEvents|InputAxisMoveForward
  (params (AxisValue :type Float%20%28single-precision%29))
  (Pawn|Input|AddMovementInput (Math|Vector|GetForwardVector (Math|Rotator|MakeRotator 0.0 0.0 (.Yaw (Math|Rotator|BreakRotator (Pawn|GetControlRotation :!class /Script/Engine.Pawn))))) AxisValue false))

(event Input|AxisEvents|InputAxisMoveRight
  (params (AxisValue :type Float%20%28single-precision%29))
  (Pawn|Input|AddMovementInput (Math|Vector|GetRightVector (Math|Rotator|MakeRotator 0.0 0.0 (.Yaw (Math|Rotator|BreakRotator (Pawn|GetControlRotation :!class /Script/Engine.Pawn))))) AxisValue false))

(fn ConstructionScript)

(fn SetCharacterWalkSpeed
  (bind _charactermovement (Variables|Character|GetCharacterMovement))
  (if (Math|Boolean|ORBoolean (Variables|Default|GetbCrouchPressed) (Variables|Default|GetbWalkPressed) (Variables|Default|GetbAimPressed))
    (Variables|/Script/Engine.CharacterMovementComponent|SetMaxWalkSpeed _charactermovement 2e+02)
    (elif (Variables|Default|GetbSprintPressed)
      (Variables|/Script/Engine.CharacterMovementComponent|SetMaxWalkSpeed _charactermovement 1e+03)
      (else
        (Variables|/Script/Engine.CharacterMovementComponent|SetMaxWalkSpeed _charactermovement 6e+02)))))

(fn Fire
  (params (AttackRange :type Integer) (LeftAmmo :type Integer))
  (bind _camera (Variables|Default|GetCamera))
  (bind _returnvalue (Transformation|GetWorldLocation _camera))
  (if (> LeftAmmo 0)
    (Utilities|FlowControl|Sequence
      (:then_0
        (Animation|Montage|MontagePlay (Components|SkeletalMesh|GetAnimInstance (Variables|Character|GetMesh)) 0 1.0 "MontageLength" 0.0 true))
      (:then_1
        (CameraShakes|StartCameraShake (Game|GetPlayerCameraManager 0) 0 1.0 "CameraLocal" "0, 0, 0"))
      (:then_2
        (Effects|SpawnEmitteratLocation "/Game/WeaponEffects/P_AssaultRifle_IH.P_AssaultRifle_IH" "0, 0, 0"))
      (:then_3
        (Audio|PlaySound2D "/Game/MilitaryWeapSilver/Sound/Rifle/Cues/RifleA_Fire_Cue.RifleA_Fire_Cue" 1.0 1.0 0.0 0 0))
      (:then_4
        (bind (_outhit _returnvalue_2) (Collision|LineTraceByChannel _returnvalue (+ _returnvalue (* (Math|Vector|GetForwardVector (Pawn|GetControlRotation :!class /Script/Engine.Pawn)) AttackRange)) "TraceTypeQuery1" false 0 "Persistent"))
        (if _returnvalue_2
          (Game|Damage|ApplyDamage (.HitActor (Collision|BreakHitResult _outhit)) 4e+01 0 self)))
      (:then_5
        (return)))
    (else
      (Audio|PlaySound2D "/Game/MilitaryWeapSilver/Sound/Rifle/Cues/Rifle_AmmoPickup_Cue.Rifle_AmmoPickup_Cue" 1.0 1.0 0.0 0 0))))