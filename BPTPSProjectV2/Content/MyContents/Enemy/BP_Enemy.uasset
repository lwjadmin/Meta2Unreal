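; BP_Enemy is a melee enemy character with a randomized mesh and gendered hurt and death sounds.
; Tick checks range to the player, looping an attack montage, or a roar once the player is dead, while ApplyPlayerDamage deals random radial damage.
; PointDamage spawns impact effects and reduces HP, ragdolling the enemy at zero and incrementing the player's kill count.
; The construction script derives mesh and gender from separate Random calls, so they can mismatch.
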(event Custom|ApplyPlayerDamage
  (bind _self self)
  (Game|Damage|ApplyRadialDamage (Math|Random|RandomFloatinRange (Variables|Default|GetMinAttackDamage) (Variables|Default|GetMaxAttackDamage)) (Transformation|GetActorLocation _self) (Variables|Default|GetAttackRange) 0 0 _self 0 true "ECC_Visibility"))

(event EventBeginPlay
  (Utilities|FlowControl|Sequence
    (:then_0
      (bind _outactors (Actor|GetAllActorsOfClass "/Game/MyContents/Player/BP_Player.BP_Player_C"))
      (for (_array_element _array_index) _outactors
        (if (== _array_index 0)
          (Variables|Default|SetRefPlayer _array_element))))
    (:then_1
      (CallFunction|UpdateCharacterWalkSpeed 2e+02))))

(event EventTick
  (params (DeltaSeconds :type Float%20%28single-precision%29))
  (bind _mesh (Variables|Character|GetMesh))
  (if (and (Utilities|Enum|NotEqual(Enum) (Variables|Default|GetEnemyStatus) "NewEnumerator3") (<= (Math|Vector|VectorLength (- (Transformation|GetActorLocation (Game|GetPlayerCharacter 0)) (Transformation|GetActorLocation self))) (Variables|Default|GetAttackRange)))
    (Variables|Default|SetEnemyStatus "NewEnumerator2")
    (Utilities|FlowControl|DoOnce false :!label _label
      (:Completed
        (if (Variables|/Game/MyContents/Player/BP_Player.BP_Player_C|GetbIsDead (Variables|Default|GetRefPlayer))
          (Animation|Montage|PlayMontage _mesh "/Game/MyContents/Enemy/AMT_Enemy_Roar.AMT_Enemy_Roar"
            (:OnCompleted
              (goto _label Reset)))
          (else
            (Animation|Montage|PlayMontage _mesh "/Game/MyContents/Enemy/AMT_Enemy_Attack.AMT_Enemy_Attack"
              (:OnCompleted
                (goto _label Reset)))))))
    (else
      (Variables|Default|SetEnemyStatus "NewEnumerator0"))))

(event Game|Damage|EventPointDamage
  (params (Damage :type Float%20%28single-precision%29) (DamageType :type Damage%20Type%20Object%20Reference) (HitLocation :type Vector :default "0, 0, 0") (HitNormal :type Vector :default "0, 0, 0") (HitComponent :type Primitive%20Component%20Object%20Reference) (BoneName :type Name :default "None") (ShotFromDirection :type Vector :default "0, 0, 0") (InstigatedBy :type Controller%20Object%20Reference) (DamageCauser :type Actor%20Object%20Reference) (HitInfo :type Hit%20Result%20Structure%20%28by%20ref%29))
  (bind _refplayer (Variables|Default|GetRefPlayer))
  (bind _mesh (Variables|Character|GetMesh))
  (Utilities|FlowControl|Sequence
    (:then_0
      (Effects|SpawnEmitteratLocation "/Game/WeaponEffects/P_body_bullet_impact.P_body_bullet_impact" ShotFromDirection)
      (Variables|Default|SetDamagePoint BoneName))
    (:then_1
      (if (not (Variables|Default|GetbIsDead))
        (bind _output_get (Variables|Default|SetbIsDead (<= (- (Variables|Default|GetCurHP) Damage) 0.0)))
        (if _output_get
          (Variables|Default|SetCurHP 0.0)
          (Variables|Default|SetEnemyStatus "NewEnumerator3")
          (Physics|SetSimulatePhysics (Variables|Character|GetMesh) true)
          (Collision|SetCollisionEnabled (Variables|Collision|GetCapsuleComponent) "NoCollision")
          (if (Variables|Default|GetbIsMale)
            (Audio|PlaySound2D "/Game/MyContents/Enemy/SC_M_EnemyDead.SC_M_EnemyDead" 1.0 1.0 0.0 0 0)
            (else
              (Audio|PlaySound2D "/Game/MyContents/Enemy/SC_FM_EnemyDead.SC_FM_EnemyDead" 1.0 1.0 0.0 0 0)))
          (Variables|/Game/MyContents/Player/BP_Player.BP_Player_C|SetEnemyKillCount _refplayer (+ (Variables|/Game/MyContents/Player/BP_Player.BP_Player_C|GetEnemyKillCount _refplayer) 1))
          (else
            (Variables|Default|SetCurHP (- (Variables|Default|GetCurHP) Damage))
            (if (Variables|Default|GetbIsMale)
              (Audio|PlaySound2D "/Game/MyContents/Enemy/SC_M_EnemyDamage.SC_M_EnemyDamage" 1.0 1.0 0.0 0 0)
              (Animation|Montage|PlayMontage _mesh 0)
              (else
                (Audio|PlaySound2D "/Game/MyContents/Enemy/SC_FM_EnemyDamage.SC_FM_EnemyDamage" 1.0 1.0 0.0 0 0)
                (Animation|Montage|PlayMontage _mesh 0)))))))))

(fn ConstructionScript
  (bind _enemymeshlist (Variables|Default|GetEnemyMeshList))
  (bind (_outitem _outindex) (Utilities|Array|Random _enemymeshlist))
  (Class|SkinnedMeshComponent|SetSkeletalMesh (Variables|Character|GetMesh) _outitem true)
  (Variables|Default|SetbIsMale (== _outindex 0)))

(fn UpdateCharacterWalkSpeed
  (params (Speed :type Float%20%28single-precision%29))
  (Variables|/Script/Engine.CharacterMovementComponent|SetMaxWalkSpeed (Variables|Character|GetCharacterMovement) Speed))