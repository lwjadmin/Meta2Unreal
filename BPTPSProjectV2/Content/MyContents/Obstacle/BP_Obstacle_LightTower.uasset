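; Light tower obstacle with four spotlights and matching bulb spheres that can be switched and spun.
; Construction tints the spotlights with LightColor and gives all spheres one shared emissive dynamic material of that color.
; LightsOnOff reapplies the tint and sets spotlight intensity to LightIntensity or zero; its bulb loop is empty, so emissive ignores the state.
; RotationOnOff sets a flag that makes Tick rotate Scene by a fixed, frame-rate-dependent step.
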(event EventBeginPlay
  (Utilities|FlowControl|Sequence
    (:then_0
      (Utilities|Array|Add (Variables|Default|GetLightList) (Variables|Default|GetSpotLight))
      (Utilities|Array|Add (Variables|Default|GetLightList) (Variables|Default|GetSpotLight1))
      (Utilities|Array|Add (Variables|Default|GetLightList) (Variables|Default|GetSpotLight2))
      (Utilities|Array|Add (Variables|Default|GetLightList) (Variables|Default|GetSpotLight3)))
    (:then_1
      (Utilities|Array|Add (Variables|Default|GetLightBulbList) (Variables|Default|GetSphere))
      (Utilities|Array|Add (Variables|Default|GetLightBulbList) (Variables|Default|GetSphere1))
      (Utilities|Array|Add (Variables|Default|GetLightBulbList) (Variables|Default|GetSphere2))
      (Utilities|Array|Add (Variables|Default|GetLightBulbList) (Variables|Default|GetSphere3)))))

(event EventTick
  (params (DeltaSeconds :type Float%20%28single-precision%29))
  (if (Variables|Default|GetbRotate)
    (Transformation|AddRelativeRotation (Variables|Default|GetScene) "0,1.000000, 0" false false)))

(fn ConstructionScript
  (CallFunction|InitLightsonOff false))

(fn LightsonOff
  (params (bDoLightsOn :type Boolean))
  (Utilities|FlowControl|Sequence
    (:then_0
      (CallFunction|InitLightsonOff bDoLightsOn))
    (:then_1
      (for _array_element (Variables|Default|GetLightList)
        (if bDoLightsOn
          (Rendering|Components|Light|SetIntensity _array_element (Variables|Default|GetLightIntensity))
          (else
            (Rendering|Components|Light|SetIntensity _array_element 0.0))))
      (for _array_element_2 (Variables|Default|GetLightBulbList)
        (if bDoLightsOn
          _)))))

(fn RotationonOff
  (params (bDoRotate :type Boolean))
  (Variables|Default|SetbRotate bDoRotate))

(fn InitLightsonOff
  (params (bIsOn :type Boolean))
  (bind _lightcolor (Variables|Default|GetLightColor))
  (Utilities|FlowControl|Sequence
    (:then_1
      (bind _returnvalue (Rendering|Material|CreateDynamicMaterialInstance "/Game/MyContents/Obstacle/M_ObstacleBase_Emissive_RGB.M_ObstacleBase_Emissive_RGB" "None" "None" :!class /Script/Engine.KismetMaterialLibrary))
      (Rendering|Material|SetVectorParameterValue _returnvalue "EmissiveColor" _lightcolor :!class /Script/Engine.MaterialInstanceDynamic)
      (Rendering|Material|SetMaterial (Variables|Default|GetSphere) 0 _returnvalue)
      (Rendering|Material|SetMaterial (Variables|Default|GetSphere1) 0 _returnvalue)
      (Rendering|Material|SetMaterial (Variables|Default|GetSphere2) 0 _returnvalue)
      (Rendering|Material|SetMaterial (Variables|Default|GetSphere3) 0 _returnvalue))
    (:then_2
      (Rendering|Components|Light|SetLightColor (Variables|Default|GetSpotLight) _lightcolor true)
      (Rendering|Components|Light|SetLightColor (Variables|Default|GetSpotLight1) _lightcolor true)
      (Rendering|Components|Light|SetLightColor (Variables|Default|GetSpotLight2) _lightcolor true)
      (Rendering|Components|Light|SetLightColor (Variables|Default|GetSpotLight3) _lightcolor true))))