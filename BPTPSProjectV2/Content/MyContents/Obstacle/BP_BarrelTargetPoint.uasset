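; BP_BarrelTargetPoint is an obstacle marker with a sphere mesh and a light bulb that can be switched on and off.
; The construction script creates a dynamic emissive material, tints it with LightColor and applies it to the sphere.
; TurnOnLights applies LightIntensity and LightColor to the bulb, while TurnOffLights zeroes intensity and resets the color.
; The event graph is empty, and neither light function is called within this Blueprint.
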(event EventBeginPlay)

(event Collision|EventActorBeginOverlap
  (params (OtherActor :type Actor%20Object%20Reference)))

(event EventTick
  (params (DeltaSeconds :type Float%20%28single-precision%29)))

(fn ConstructionScript
  (bind _returnvalue (Rendering|Material|CreateDynamicMaterialInstance "/Game/MyContents/Obstacle/M_ObstacleBase_Emissive_RGB.M_ObstacleBase_Emissive_RGB" "None" "None" :!class /Script/Engine.KismetMaterialLibrary))
  (bind _output_get (Variables|Default|SetMI_SphereMesh _returnvalue))
  (Utilities|IsValid _output_get
    (:Is%20Valid
      (Rendering|Material|SetVectorParameterValue (Variables|Default|GetMI_SphereMesh) "EmissiveColor" (Variables|Default|GetLightColor) :!class /Script/Engine.MaterialInstanceDynamic)
      (Rendering|Material|SetMaterial (Variables|Default|GetSphereMesh) 0 (Variables|Default|GetMI_SphereMesh)))))

(fn TurnonLights
  (bind _lightbulb (Variables|Default|GetLightBulb))
  (Rendering|Components|Light|SetIntensity _lightbulb (Variables|Default|GetLightIntensity))
  (Rendering|Components|Light|SetLightColor _lightbulb (Variables|Default|GetLightColor) true))

(fn TurnOffLights
  (bind _lightbulb (Variables|Default|GetLightBulb))
  (Rendering|Components|Light|SetIntensity _lightbulb 0.0)
  (Rendering|Components|Light|SetLightColor _lightbulb (Utilities|Struct|MakeLinearColor 0.0 0.0 0.0 0.0) true))