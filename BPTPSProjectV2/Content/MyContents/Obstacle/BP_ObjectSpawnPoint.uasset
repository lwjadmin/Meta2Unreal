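; Obstacle spawn point actor with a light that can switch on and off; only the lighting logic is present here.
; LightOnOff drives an emissive dynamic material on LightMesh and the LightBulb intensity from default color and intensity, creating the material instance on demand.
; The construction script applies the default state.
; Tick switches the light off after AutoLightsOffDelaySeconds, when that delay is positive.
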(event EventTick
  (params (DeltaSeconds :type Float%20%28single-precision%29))
  (if (and (Variables|Default|GetbIsOn) (> (Variables|Default|GetAutoLightsOffDelaySeconds) 0.0))
    (bind _output_get (Variables|Default|SetLightOnElapsedSeconds (+ (Variables|Default|GetLightOnElapsedSeconds) DeltaSeconds)))
    (if (> _output_get (Variables|Default|GetAutoLightsOffDelaySeconds))
      (CallFunction|LightonOff false)
      (Variables|Default|SetLightOnElapsedSeconds 0.0))))

(fn ConstructionScript
  (CallFunction|LightonOff (Variables|Default|GetbDefaultLightIsOn)))

(fn LightonOff
  (params (LightOn :type Boolean))
  (bind _lightbulb (Variables|Default|GetLightBulb))
  (Utilities|IsValid (Variables|Default|GetMI_LightMesh)
    (:Is%20Valid
      _)
    (:Is%20Not%20Valid
      (bind _returnvalue (Rendering|Material|CreateDynamicMaterialInstance "/Game/MyContents/Obstacle/M_ObstacleBase_Emissive_RGB.M_ObstacleBase_Emissive_RGB" "None" "None" :!class /Script/Engine.KismetMaterialLibrary))
      (Variables|Default|SetMI_LightMesh _returnvalue)))
  (if LightOn
    (Rendering|Material|SetScalarParameterValue (Variables|Default|GetMI_LightMesh) "ScaleX" 0.75 :!class /Script/Engine.MaterialInstanceDynamic)
    (Rendering|Material|SetScalarParameterValue (Variables|Default|GetMI_LightMesh) "ScaleY" 0.75 :!class /Script/Engine.MaterialInstanceDynamic)
    (Rendering|Material|SetVectorParameterValue (Variables|Default|GetMI_LightMesh) "EmissiveColor" (* (Variables|Default|GetDefaultLightColor) (Variables|Default|GetDefaultLightIntensity)) :!class /Script/Engine.MaterialInstanceDynamic)
    (Rendering|Material|SetMaterial (Variables|Default|GetLightMesh) 0 (Variables|Default|GetMI_LightMesh))
    (Rendering|Components|Light|SetIntensity _lightbulb (* (Variables|Default|GetDefaultLightIntensity) 1e+02))
    (Rendering|Components|Light|SetLightColor _lightbulb (Variables|Default|GetDefaultLightColor) true)
    (else
      (Rendering|Material|SetScalarParameterValue (Variables|Default|GetMI_LightMesh) "ScaleX" 0.75 :!class /Script/Engine.MaterialInstanceDynamic)
      (Rendering|Material|SetScalarParameterValue (Variables|Default|GetMI_LightMesh) "ScaleY" 0.75 :!class /Script/Engine.MaterialInstanceDynamic)
      (Rendering|Material|SetVectorParameterValue (Variables|Default|GetMI_LightMesh) "EmissiveColor" (Variables|Default|GetDefaultLightColor) :!class /Script/Engine.MaterialInstanceDynamic)
      (Rendering|Material|SetMaterial (Variables|Default|GetLightMesh) 0 (Variables|Default|GetMI_LightMesh))
      (Rendering|Components|Light|SetIntensity (Variables|Default|GetLightBulb) (* (Variables|Default|GetDefaultLightIntensity) 0.0))))
  (Variables|Default|SetbIsOn LightOn))