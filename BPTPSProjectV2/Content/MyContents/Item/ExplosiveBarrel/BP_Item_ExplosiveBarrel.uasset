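; Explosive barrel item that takes point damage from the player and explodes when its randomized health runs out.
; Construction picks a random mesh, and BeginPlay rolls health and adds an "Explosion" tag.
; Non-lethal hits play impact effects, using the shot direction as the emitter location.
; The lethal hit plays explosion effects, applies radial damage with amount and radius both rolled from the attack range bounds, then destroys the barrel.
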(event EventBeginPlay
  (Variables|Default|SetCurHP (Math|Random|RandomFloatinRange (Variables|Default|GetMinHP) (Variables|Default|GetMaxHP)))
  (Variables|Default|SetTags self (Utilities|Array|MakeArray "Explosion")))

(event Game|Damage|EventPointDamage
  (params (Damage :type Float%20%28single-precision%29) (DamageType :type Damage%20Type%20Object%20Reference) (HitLocation :type Vector :default "0, 0, 0") (HitNormal :type Vector :default "0, 0, 0") (HitComponent :type Primitive%20Component%20Object%20Reference) (BoneName :type Name :default "None") (ShotFromDirection :type Vector :default "0, 0, 0") (InstigatedBy :type Controller%20Object%20Reference) (DamageCauser :type Actor%20Object%20Reference) (HitInfo :type Hit%20Result%20Structure%20%28by%20ref%29))
  (Utilities|Casting|CastToBP_Player DamageCauser)
  (if (not (Variables|Default|GetbIsDestroyed))
    (bind _output_get (Variables|Default|SetbIsDestroyed (<= (- (Variables|Default|GetCurHP) Damage) 0.0)))
    (if _output_get
      (Audio|PlaySoundatLocation "/Game/MilitaryWeapSilver/Sound/RocketLauncher/Cues/RocketLauncher_Explosion_Cue.RocketLauncher_Explosion_Cue" (Transformation|GetActorLocation self) "0, 0, 0" 1.0 1.0 0.0 0 0 0)
      (Effects|SpawnEmitteratLocation "/Game/MilitaryWeapSilver/FX/P_RocketLauncher_Explosion_01.P_RocketLauncher_Explosion_01" (Transformation|GetActorLocation self))
      (Game|Damage|ApplyRadialDamage (Math|Random|RandomFloatinRange (Variables|Default|GetMinAttackRange) (Variables|Default|GetMaxAttackRange)) (Transformation|GetActorLocation self) (Math|Random|RandomFloatinRange (Variables|Default|GetMinAttackRange) (Variables|Default|GetMaxAttackRange)) 0 0 self 0 false "ECC_Visibility")
      (Actor|DestroyActor)
      (else
        (Variables|Default|SetCurHP (- (Variables|Default|GetCurHP) Damage))
        (Effects|SpawnEmitteratLocation "/Game/MilitaryWeapSilver/FX/P_Impact_Metal_Large_01.P_Impact_Metal_Large_01" ShotFromDirection)
        (Audio|PlaySoundatLocation "/Game/MilitaryWeapSilver/Sound/Rifle/Cues/Rifle_ImpactSurface_Cue.Rifle_ImpactSurface_Cue" (Transformation|GetActorLocation self) "0, 0, 0" 1.0 1.0 0.0 0 0 0)))))

(fn ConstructionScript
  (Components|StaticMesh|SetStaticMesh (Variables|Default|GetSM_Barrel) (.OutItem (Utilities|Array|Random (Variables|Default|GetBarrelMeshList)))))