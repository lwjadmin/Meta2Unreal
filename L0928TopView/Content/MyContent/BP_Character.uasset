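; Player character Blueprint for cursor-driven movement, with a visible mouse cursor and a Jump action.
; Holding the left mouse button opens a gate that, each Tick, sends the controller toward the point under the cursor via SimpleMoveToLocation.
; Tick also moves a decal to the cursor's Visibility trace hit, oriented to the surface normal.
; WASD and mouse-look events are empty, their movement and rotation nodes left unconnected.
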(event EventBeginPlay
  ;[1 1 1] show mouse cursor
  (Variables|/Script/Engine.PlayerController|SetbShowMouseCursor (Game|GetPlayerController 0) true))

(event EventTick
  (params (DeltaSeconds :type Float%20%28single-precision%29))
  (bind _returnvalue (Game|GetPlayerController 0))
  (bind _hitresult (Game|Player|GetHitResultUnderCursorbyChannel _returnvalue "TraceTypeQuery1" true))
  ;[1 1 1] Move to Clicked Mouse Cursor Position
  (Utilities|FlowControl|Sequence
    (:then_0
      (Utilities|FlowControl|Gate true
        (:Exit
          (if true
            (AI|Navigation|SimpleMovetoLocation _returnvalue (.location _hitresult))))))
    (:then_1
      (Transformation|SetWorldLocationAndRotation (Variables|Default|GetDecal) (.location _hitresult) (Math|Rotator|MakeRotationfromAxes (.impactnormal _hitresult) "0, 0, 0" "0, 0, 0") false false))))

(event Input|ActionEvents|InputActionJump
  (params (Key :type Key%20Structure :default "None"))
  ;[1 1 1] OtherActions
  (:Pressed
    (Character|Jump))
  (:Released
    (Character|StopJumping)))

(event Input|AxisEvents|InputAxisMoveForward
  (params (AxisValue :type Float%20%28single-precision%29))
  ;[1 1 1] WASD
)

(event Input|AxisEvents|InputAxisMoveRight
  (params (AxisValue :type Float%20%28single-precision%29))
  ;[1 1 1] WASD
)

(event Input|AxisEvents|InputAxisTurn
  (params (AxisValue :type Float%20%28single-precision%29))
  ;[1 1 1] MouseXY
)

(event Input|AxisEvents|InputAxisLookUp
  (params (AxisValue :type Float%20%28single-precision%29))
  ;[1 1 1] MouseXY
)

(event Input|MouseEvents|LeftMouseButton
  (params (Key :type Key%20Structure :default "None"))
  (bind _returnvalue (Game|GetPlayerController 0))
  ;[1 1 1] Move to Clicked Mouse Cursor Position
  (:Pressed
    (Utilities|FlowControl|Gate true) ; enters at Open
  )
  (:Released
    (Utilities|FlowControl|Gate true) ; enters at Close
  ))

(fn ConstructionScript)