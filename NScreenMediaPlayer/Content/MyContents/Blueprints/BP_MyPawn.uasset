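; Player pawn that flies around relative to the camera and acts as a remote control for media players in the level.
; Move axes offset the actor along camera forward and right vectors without sweeping; LookUp feeds yaw and LookLeftRight feeds pitch, opposite to their names.
; Play/stop (toggled by a Stopped flag), forward, backward and volume inputs broadcast BPI_MediaPlayer messages to every implementing actor, found afresh on each press.
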(event Input|ActionEvents|InputActionPlay_Stop
  (params (Key :type Key%20Structure :default "None"))
  (:Pressed
    (if (Variables|Default|GetbStopped)
      (bind _outactors (Actor|GetAllActorswithInterface "/Game/MyContents/Blueprints/BPI_MediaPlayer.BPI_MediaPlayer_C"))
      (Variables|Default|SetbStopped false)
      (Development|PrintString "Start Called!")
      (for _array_element _outactors
        (Class|BPIMediaPlayer|BPIPlay(Message) _array_element))
      (else
        (bind _outactors_2 (Actor|GetAllActorswithInterface "/Game/MyContents/Blueprints/BPI_MediaPlayer.BPI_MediaPlayer_C"))
        (Variables|Default|SetbStopped true)
        (Development|PrintString "Stop Called!")
        (for _array_element_2 _outactors_2
          (Class|BPIMediaPlayer|BPIStop(Message) _array_element_2))))))

(event Input|ActionEvents|InputActionGoForward
  (params (Key :type Key%20Structure :default "None"))
  (:Pressed
    (Development|PrintString "Go Forward!")
    (bind _outactors (Actor|GetAllActorswithInterface "/Game/MyContents/Blueprints/BPI_MediaPlayer.BPI_MediaPlayer_C"))
    (for _array_element _outactors
      (Class|BPIMediaPlayer|BPIGoForward(Message) _array_element))))

(event Input|ActionEvents|InputActionGoBackward
  (params (Key :type Key%20Structure :default "None"))
  (:Pressed
    (Development|PrintString "Go Backward!")
    (bind _outactors (Actor|GetAllActorswithInterface "/Game/MyContents/Blueprints/BPI_MediaPlayer.BPI_MediaPlayer_C"))
    (for _array_element _outactors
      (Class|BPIMediaPlayer|BPIGoBackward(Message) _array_element))))

(event Input|ActionEvents|InputActionVolumeUp
  (params (Key :type Key%20Structure :default "None"))
  (:Pressed
    (bind _outactors (Actor|GetAllActorswithInterface "/Game/MyContents/Blueprints/BPI_MediaPlayer.BPI_MediaPlayer_C"))
    (for _array_element _outactors
      (Class|BPIMediaPlayer|BPIVolumeUp(Message) _array_element))))

(event Input|ActionEvents|InputActionVolumeDown
  (params (Key :type Key%20Structure :default "None"))
  (:Pressed
    (bind _outactors (Actor|GetAllActorswithInterface "/Game/MyContents/Blueprints/BPI_MediaPlayer.BPI_MediaPlayer_C"))
    (for _array_element _outactors
      (Class|BPIMediaPlayer|BPIVolumeDown(Message) _array_element))))

(event Input|AxisEvents|InputAxisMoveRight
  (params (AxisValue :type Float%20%28single-precision%29))
  (Transformation|AddActorWorldOffset (* (Math|Vector|GetRightVector (Variables|/Script/Engine.PlayerCameraManager|GetTransformComponent (Game|GetPlayerCameraManager 0))) (* AxisValue (Variables|Default|GetMoveSpeed)))))

(event Input|AxisEvents|InputAxisMoveForward
  (params (AxisValue :type Float%20%28single-precision%29))
  (Transformation|AddActorWorldOffset (* (Math|Vector|GetForwardVector (Variables|/Script/Engine.PlayerCameraManager|GetTransformComponent (Game|GetPlayerCameraManager 0))) (* AxisValue (Variables|Default|GetMoveSpeed)))))

(event Input|AxisEvents|InputAxisLookUp
  (params (AxisValue :type Float%20%28single-precision%29))
  (Pawn|Input|AddControllerYawInput AxisValue))

(event Input|AxisEvents|InputAxisLookLeftRight
  (params (AxisValue :type Float%20%28single-precision%29))
  (Pawn|Input|AddControllerPitchInput AxisValue))

(fn ConstructionScript)