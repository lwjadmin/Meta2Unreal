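; Media player actor that opens a media source on BeginPlay and routes its audio to a media sound component.
; Interface events play, pause, seek forward or backward by a set number of seconds, and step the volume between zero and full.
; Seeking pauses playback, waits briefly, then resumes only if BP_MyPawn is not flagged as stopped.
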(event EventBeginPlay
  (bind _targetmedia (Variables|Default|GetTargetMedia))
  (Media|MediaSoundComponent|SetMediaPlayer (Variables|Default|GetMediaSound) _targetmedia)
  (Media|MediaPlayer|OpenSource _targetmedia (Variables|Default|GetTargetMediaSource)))

(event EventBPIStop
  (bind _targetmedia (Variables|Default|GetTargetMedia))
  (if (Audio|Components|Audio|IsPlaying _targetmedia)
    (Sequencer|Player|Pause _targetmedia)))

(event EventBPIPlay
  (bind _targetmedia (Variables|Default|GetTargetMedia))
  (if (not (Audio|Components|Audio|IsPlaying _targetmedia))
    (Media|MediaPlayer|Play _targetmedia :!class /Script/MediaAssets.MediaPlayer)))

(event EventBPIGoBackward
  (bind _targetmedia (Variables|Default|GetTargetMedia))
  (bind _returnvalue (Class|MediaPlayer|GetTime _targetmedia))
  (Sequencer|Player|Pause _targetmedia)
  (Media|MediaPlayer|Seek _targetmedia (Math|Timespan|MakeTimespan (.days _returnvalue) (.hours _returnvalue) (.minutes _returnvalue) (- (.seconds _returnvalue) (Variables|Default|GetSeekSecond)) (.milliseconds _returnvalue)))
  (Utilities|FlowControl|Delay 0.2)
  (bind _returnvalue_2 (Actor|GetActorOfClass "/Game/MyContents/Blueprints/BP_MyPawn.BP_MyPawn_C"))
  (if (not (Variables|/Game/MyContents/Blueprints/BP_MyPawn.BP_MyPawn_C|GetbStopped _returnvalue_2))
    (Media|MediaPlayer|Play _targetmedia :!class /Script/MediaAssets.MediaPlayer)))

(event EventBPIGoForward
  (bind _targetmedia (Variables|Default|GetTargetMedia))
  (bind _returnvalue (Class|MediaPlayer|GetTime _targetmedia))
  (Sequencer|Player|Pause _targetmedia)
  (Media|MediaPlayer|Seek _targetmedia (Math|Timespan|MakeTimespan (.days _returnvalue) (.hours _returnvalue) (.minutes _returnvalue) (+ (.seconds _returnvalue) (Variables|Default|GetSeekSecond)) (.milliseconds _returnvalue)))
  (Utilities|FlowControl|Delay 0.2)
  (bind _returnvalue_2 (Actor|GetActorOfClass "/Game/MyContents/Blueprints/BP_MyPawn.BP_MyPawn_C"))
  (if (not (Variables|/Game/MyContents/Blueprints/BP_MyPawn.BP_MyPawn_C|GetbStopped _returnvalue_2))
    (Media|MediaPlayer|Play _targetmedia :!class /Script/MediaAssets.MediaPlayer)))

(event EventBPIVolumeUp
  (if (< (Variables|Default|GetVolume) 1.0)
    (bind _output_get (Variables|Default|SetVolume (+ (Variables|Default|GetVolume) 0.1)))
    (Audio|Components|Audio|SetVolumeMultiplier (Variables|Default|GetMediaSound) _output_get :!class /Script/AudioMixer.SynthComponent)))

(event EventBPIVolumeDown
  (if (> (Variables|Default|GetVolume) 0.0)
    (bind _output_get (Variables|Default|SetVolume (- (Variables|Default|GetVolume) 0.1)))
    (Audio|Components|Audio|SetVolumeMultiplier (Variables|Default|GetMediaSound) _output_get :!class /Script/AudioMixer.SynthComponent)))

(fn ConstructionScript)