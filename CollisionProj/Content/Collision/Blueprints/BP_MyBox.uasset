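; BP_MyBox is a collision test box that relays Cube2's begin and end overlaps through event dispatchers.
; Overlap and hit handlers also build debug strings, but their screen and log output is switched off.
; The remaining graph is unreached practice code: loops, lazy BPI_Move actor lookup with Play/Stop messaging, and helpers that gather actors by name prefix or mover class casts.
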(event OnComponentBeginOverlap(Cube2)
  (params (OverlappedComponent :type Primitive%20Component%20Object%20Reference) (OtherActor :type Actor%20Object%20Reference) (OtherComp :type Primitive%20Component%20Object%20Reference) (OtherBodyIndex :type Integer) (bFromSweep :type Boolean) (SweepResult :type Hit%20Result%20Structure%20%28by%20ref%29))
  (Development|PrintString (Utilities|String|Append "Overlapped Component : " (Utilities|GetDisplayName OverlappedComponent) ", Other Actor :" (Utilities|GetDisplayName OtherActor) ", Other Comp : " (Utilities|GetDisplayName OtherComp)) false false "(R=0.000000,G=0.660000,B=1.000000,A=1.000000)" 2e+02)
  (Default|CallEventDispatcherBeginOverlap false))

(event OnComponentEndOverlap(Cube2)
  (params (OverlappedComponent :type Primitive%20Component%20Object%20Reference) (OtherActor :type Actor%20Object%20Reference) (OtherComp :type Primitive%20Component%20Object%20Reference) (OtherBodyIndex :type Integer))
  (Development|PrintString (Utilities|String|Append "End Overlapped Component : " (Utilities|GetDisplayName OverlappedComponent) ", Other Actor :" (Utilities|GetDisplayName OtherActor) ", Other Comp : " (Utilities|GetDisplayName OtherComp)) false false "(R=0.000000,G=0.660000,B=1.000000,A=1.000000)" 2e+02)
  (Default|CallEventDispatcherEndOverlap))

(event OnComponentHit(Cube2)
  (params (HitComponent :type Primitive%20Component%20Object%20Reference) (OtherActor :type Actor%20Object%20Reference) (OtherComp :type Primitive%20Component%20Object%20Reference) (NormalImpulse :type Vector :default "0, 0, 0") (Hit :type Hit%20Result%20Structure%20%28by%20ref%29))
  (Development|PrintString (Utilities|String|Append "Hit Component : " (Utilities|GetDisplayName HitComponent) ", Other Actor :" (Utilities|GetDisplayName OtherActor) ", Other Comp : " (Utilities|GetDisplayName OtherComp)) false false "(R=0.000000,G=0.660000,B=1.000000,A=1.000000)" 2e+02))

(event EventBeginPlay)

(fn ConstructionScript)

(fn FindActorsbyLabel
  (params (Keyword :type Array%20of%20Strings) (ActorRef :type Array%20of%20Actor%20Object%20References))
  (bind _outactors (Actor|GetAllActorsOfClass "/Script/Engine.Actor"))
  (for _array_element _outactors
    (for _array_element_2 Keyword
      (if (Utilities|String|StartsWith (Utilities|GetDisplayName _array_element) _array_element_2)
        (Utilities|Array|Add ActorRef _array_element)))))

(fn FindActorsbyExactClass
  (params (ActorRef :type Array%20of%20Actor%20Object%20References))
  (bind _outactors (Actor|GetAllActorsOfClass "/Script/Engine.Actor"))
  (for _array_element _outactors
    (bind _asbp_move_left_right (Utilities|Casting|CastToBP_MoveLeftRight _array_element)
      (:then
        (Utilities|Array|Add ActorRef _asbp_move_left_right))
      (:CastFailed
        (bind _asbp_move_rect (Utilities|Casting|CastToBP_MoveRect _array_element)
          (:then
            (Utilities|Array|Add ActorRef _asbp_move_rect))
          (:CastFailed
            (bind _asbp_rotation_ball (Utilities|Casting|CastToBP_RotationBall _array_element))
            (Utilities|Array|Add ActorRef _asbp_rotation_ball)))))))