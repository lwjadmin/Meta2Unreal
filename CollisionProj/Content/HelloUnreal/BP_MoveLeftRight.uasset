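; BP_MoveLeftRight is a Blueprint that slides its static mesh back and forth along relative X using a timeline.
; On BeginPlay it binds events to the begin and end overlap dispatchers of every BP_MyBox in the level.
; The begin-overlap handler calls Play, which plays or reverses the timeline by a direction flag, flipping it on each finish to loop.
; A Stop event halts the timeline.
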(event Custom|커스텀이벤트_0)

(event EventPlay
  (if (Variables|Default|GetisMoveRight) :!label _label
    (bind _fval (Timeline|타임라인_0 Play)
      (:Update
        (Transformation|SetRelativeLocation (Variables|Default|GetStaticMesh) (Math|Vector|MakeVector (* _fval 1e+03) 0.0 0.0) false false))
      (:Finished
        (Variables|Default|SetisMoveRight (not (Variables|Default|GetisMoveRight)))
        (goto _label)))
    (else
      (Timeline|타임라인_0 Reverse))))

(event EventStop
  (bind _fval (Timeline|타임라인_0 Stop)
    (:Update
      (Transformation|SetRelativeLocation (Variables|Default|GetStaticMesh) (Math|Vector|MakeVector (* _fval 1e+03) 0.0 0.0) false false))
    (:Finished
      (Variables|Default|SetisMoveRight (not (Variables|Default|GetisMoveRight)))
      (if (Variables|Default|GetisMoveRight)
        (Timeline|타임라인_0 Play)
        (else
          (Timeline|타임라인_0 Reverse))))))

(event EventBeginPlay
  (bind _outactors (Actor|GetAllActorsOfClass "/Game/Collision/Blueprints/BP_MyBox.BP_MyBox_C"))
  (for _array_element _outactors
    (Utilities|FlowControl|Sequence
      (:then_0
        (EventDispatchers|BindEventtoEventDispatcherBeginOverlap _array_element (EventDispatchers|CreateEvent :!event EVentBeginOverlap)))
      (:then_1
        (EventDispatchers|BindEventtoEventDispatcherEndOverlap _array_element (EventDispatchers|CreateEvent :!event Stop))))))

(fn ConstructionScript)

(fn EVentBeginOverlap
  (params (bResult :type Boolean))
  (CallFunction|Play))