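; BP_RotationBall is an actor whose Scene component swings on its roll axis, with Play and Stop events to control the motion.
; On BeginPlay it binds events to the begin and end overlap dispatchers of every BP_MyBox in the level.
; Play runs a timeline that drives the roll, flipping IsNodeRight on each finish to alternate forward and reverse playback, while Stop halts it.
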(event EventPlay
  (if (Variables|Default|GetisNodeRight) :!label _label
    (bind _value (Timeline|타임라인_0 Play)
      (:Update
        (Transformation|SetRelativeRotation (Variables|Default|GetScene) (Math|Rotator|MakeRotator (* _value 45.0) 0.0 0.0) false false))
      (:Finished
        (Variables|Default|SetisNodeRight (not (Variables|Default|GetisNodeRight)))
        (goto _label)))
    (else
      (Timeline|타임라인_0 Reverse))))

(event EventStop
  (bind _value (Timeline|타임라인_0 Stop)
    (:Update
      (Transformation|SetRelativeRotation (Variables|Default|GetScene) (Math|Rotator|MakeRotator (* _value 45.0) 0.0 0.0) false false))
    (:Finished
      (Variables|Default|SetisNodeRight (not (Variables|Default|GetisNodeRight)))
      (if (Variables|Default|GetisNodeRight)
        (Timeline|타임라인_0 Play)
        (else
          (Timeline|타임라인_0 Reverse))))))

(event EventBeginPlay
  (bind _outactors (Actor|GetAllActorsOfClass "/Game/Collision/Blueprints/BP_MyBox.BP_MyBox_C"))
  (for _array_element _outactors
    (Utilities|FlowControl|Sequence
      (:then_0
        (EventDispatchers|BindEventtoEventDispatcherBeginOverlap _array_element (EventDispatchers|CreateEvent :!event BPRotationBallAutoGenFunc)))
      (:then_1
        (EventDispatchers|BindEventtoEventDispatcherEndOverlap _array_element (EventDispatchers|CreateEvent :!event Stop))))))

(fn ConstructionScript)

(fn BPRotationBallAutoGenFunc
  (params (bResult :type Boolean))
  (CallFunction|Play))