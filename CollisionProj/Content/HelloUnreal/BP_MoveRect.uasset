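; BP_MoveRect is an actor that moves its static mesh around a rectangular loop in the relative X-Z plane.
; On BeginPlay it binds handlers to the begin and end overlap dispatchers of every BP_MyBox.
; Play and Stop start and clear a fast looping timer on UpdateMove.
; UpdateMove is a MoveType state machine, stepping the mesh a fixed amount per tick and switching direction at each bound.
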(event EventPlay
  (Utilities|Time|SetTimerbyFunctionName 0 "UpdateMove" 0.01 true))

(event EventStop
  (Utilities|Time|ClearTimerbyFunctionName 0 "UpdateMove"))

(event EventBeginPlay
  (bind _outactors (Actor|GetAllActorsOfClass "/Game/Collision/Blueprints/BP_MyBox.BP_MyBox_C"))
  (for _array_element _outactors
    (Utilities|FlowControl|Sequence
      (:then_0
        (EventDispatchers|BindEventtoEventDispatcherBeginOverlap _array_element (EventDispatchers|CreateEvent :!event BPMoveRectAutoGenFunc)))
      (:then_1
        (EventDispatchers|BindEventtoEventDispatcherEndOverlap _array_element (EventDispatchers|CreateEvent :!event Stop))))))

(fn ConstructionScript)

(fn UpdateMove
  (bind _staticmesh (Variables|Default|GetStaticMesh))
  (switch Utilities|FlowControl|Switch|SwitchonEnum_MoveType (Variables|Default|GetMoveType)
    (:NewEnumerator0
      (Transformation|AddRelativeLocation _staticmesh "5.000000, 0, 0" false false)
      (if (> (.x (Variables|/Script/Engine.SceneComponent|GetRelativeLocation (Variables|Default|GetStaticMesh))) 3e+02)
        (Variables|Default|SetMoveType "NewEnumerator1")))
    (:NewEnumerator1
      (Transformation|AddRelativeLocation _staticmesh "0.000000,0.000000,5.000000" false false)
      (if (> (.z (Variables|/Script/Engine.SceneComponent|GetRelativeLocation (Variables|Default|GetStaticMesh))) 3e+02)
        (Variables|Default|SetMoveType "NewEnumerator2")))
    (:NewEnumerator2
      (Transformation|AddRelativeLocation _staticmesh "-5.000000, 0, 0" false false)
      (if (< (.x (Variables|/Script/Engine.SceneComponent|GetRelativeLocation (Variables|Default|GetStaticMesh))) 0.0)
        (Variables|Default|SetMoveType "NewEnumerator3")))
    (:NewEnumerator3
      (Transformation|AddRelativeLocation _staticmesh "0.000000, 0,-5.000000" false false)
      (if (< (.z (Variables|/Script/Engine.SceneComponent|GetRelativeLocation (Variables|Default|GetStaticMesh))) 0.0)
        (Variables|Default|SetMoveType "NewEnumerator0")))))

(fn BPMoveRectAutoGenFunc
  (params (bResult :type Boolean))
  (CallFunction|Play))