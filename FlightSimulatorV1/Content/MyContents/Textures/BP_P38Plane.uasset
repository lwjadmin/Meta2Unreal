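; BP_P38Plane is a P-38 plane Blueprint that spins its two propellers and flies along world X at a constant speed.
; Each Tick calls RotatePropeller for the left and right propellers, then offsets the actor, with both motions scaled by delta time.
; RotatePropeller adds relative roll from the RPM value without unit conversion, so it acts as degrees per second.
; BeginPlay enables player input, but the graphs contain no input events.
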(event EventBeginPlay
  (Input|EnableInput (Game|GetPlayerController 0)))

(event EventTick
  (params (DeltaSeconds :type Float%20%28single-precision%29))
  (Utilities|FlowControl|Sequence
    (:then_0
      (CallFunction|RotatePropeller (Variables|Default|GetRightPropeller) (Variables|Default|GetRPM))
      (CallFunction|RotatePropeller (Variables|Default|GetLeftPropeller) (Variables|Default|GetRPM))
      (Transformation|AddActorWorldOffset self (Math|Vector|MakeVector (* (Utilities|Time|GetWorldDeltaSeconds) 1e+02) 0.0 0.0)))))

(event Input|KeyboardEvents|D
  (params (Key :type Key%20Structure :default "None")))

(event Input|KeyboardEvents|A
  (params (Key :type Key%20Structure :default "None")))

(event Input|KeyboardEvents|W
  (params (Key :type Key%20Structure :default "None")))

(event Input|KeyboardEvents|S
  (params (Key :type Key%20Structure :default "None")))

(fn ConstructionScript)

(fn RotatePropeller
  (params (Propeller :type Static%20Mesh%20Component%20Object%20Reference) (RPM :type Float%20%28single-precision%29))
  (Transformation|AddRelativeRotation Propeller (Math|Rotator|MakeRotator (* RPM (Utilities|Time|GetWorldDeltaSeconds)) 0.0 0.0) false false)
  (return))