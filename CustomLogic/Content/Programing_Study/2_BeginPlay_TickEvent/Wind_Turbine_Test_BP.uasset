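; Test actor Blueprint for a wind turbine, used to study BeginPlay and Tick, that spins its propeller while counting elapsed seconds.
; Tick accumulates delta time, floors it to whole seconds and prints the count only when the text differs from the cached string.
; The same Tick then adds a fixed per-frame local pitch rotation to the propeller scene component, so spin speed depends on frame rate.
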(event EventBeginPlay)

(event Collision|EventActorBeginOverlap
  (params (OtherActor :type Actor%20Object%20Reference)))

(event EventTick
  (params (DeltaSeconds :type Float%20%28single-precision%29))
  (Utilities|FlowControl|Sequence
    (:then_0
      (bind _output_get (Variables|Default|SetTotalDeltaSeconds (+ (Variables|Default|GetTotalDeltaSeconds) DeltaSeconds)))
      (bind _output_get_2 (Variables|Default|SetTotalSeconds (Math|Float|Floor _output_get)))
      (if (Utilities|Enum|NotEqual(Enum) (Utilities|String|Append "TotalSeconds : " (Utilities|String|ToString(Integer) _output_get_2)) (Variables|Default|GettmpString))
        (bind _output_get_3 (Variables|Default|SettmpString (Utilities|String|Append "TotalSeconds : " (Utilities|String|ToString(Integer) _output_get_2))))
        (Development|PrintString _output_get_3 true true "(R=0.000000,G=0.660000,B=1.000000,A=1.000000)" 1.0)))
    (:then_1
      (Transformation|AddLocalRotation (Variables|Default|GetPropellerFan_Rotation_Scene) (Math|Rotator|MakeRotator 0.0 (Variables|Default|GetRotationPerFrame) 0.0) false false))))

(fn ConstructionScript)