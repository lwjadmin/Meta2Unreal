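; Wind turbine Blueprint that spins its propeller fan from an RPM variable.
; Each Tick adds local pitch to PropellerFanRotationScene, scaled by RPM, 360 over the rounded-up frame rate, and delta time.
; Delta time effectively applies twice, so spin speed varies with frame rate and is not true revolutions per minute.
; An unconnected branch that would set a random blade angle never runs.
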(event EventBeginPlay)

(event Collision|EventActorBeginOverlap
  (params (OtherActor :type Actor%20Object%20Reference)))

(event EventTick
  (params (DeltaSeconds :type Float%20%28single-precision%29))
  (Transformation|AddLocalRotation (Variables|Default|GetPropellerFan_Rotation_Scene) (Math|Rotator|MakeRotator 0.0 (* (Math|Conversions|ToFloat(Integer) (* (Variables|Default|GetRPM) (/ 360 (Math|Float|Ceil (/ 1.0 DeltaSeconds))))) DeltaSeconds) 0.0) false false))

(fn ConstructionScript)