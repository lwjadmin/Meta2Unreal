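; Player character for a third-person shooter, handling movement stances, aiming, rifle fire, ammo and health.
; Input flags set walk speed; aiming adds a crosshair widget, zooms FOV by timeline and switches rotation to controller yaw.
; A Tick-fed Gate with a Delay repeats camera line-trace shots while aiming, with montage, shake and effects.
; Damage darkens the body through a dynamic material; death turns mesh and gun to physics and disables input.
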(event Custom|EventGetAmmunition
  (Variables|Default|SetMaxAmmoCount (+ (Variables|Default|GetMaxAmmoCount) (Variables|Default|GetAmmoMagazineSize)))
  (Audio|PlaySound2D "/Game/UnrealFreeAssets/MilitaryWeapDark/Sound/Rifle/Rifle_AmmoPickup_Cue.Rifle_AmmoPickup_Cue" 1.0 1.0 0.0 0 0))

(event EventBeginPlay
  (bind _montagepool (Variables|Default|GetMontagePool))
  (Utilities|FlowControl|Sequence
    (:then_0
      (Utilities|Array|Add _montagepool "/Game/MyContents/TPSGunner/Hit_React_2_Montage.Hit_React_2_Montage")
      (Utilities|Array|Add _montagepool "/Game/MyContents/TPSGunner/Hit_React_3_Montage.Hit_React_3_Montage")
      (Utilities|Array|Add _montagepool "/Game/MyContents/TPSGunner/Hit_React_4_Montage.Hit_React_4_Montage"))
    (:then_1
      (bind _returnvalue (UserInterface|CreateWidget "/Game/MyContents/TPSGunner/UMG_TPSCharacterUI.UMG_TPSCharacterUI_C"))
      (UserInterface|Viewport|AddtoViewport _returnvalue 0))
    (:then_2
      (Variables|/Script/Engine.SpringArmComponent|SetbEnableCameraLag (Variables|Default|GetSpringArm) (Variables|Default|GetEnableCameraRotationLag)))))

(event Game|Damage|EventAnyDamage
  (params (Damage :type Float%20%28single-precision%29) (DamageType :type Damage%20Type%20Object%20Reference) (InstigatedBy :type Controller%20Object%20Reference) (DamageCauser :type Actor%20Object%20Reference))
  (bind _returnvalue (Transformation|GetActorLocation DamageCauser))
  (bind _returnvalue_2 (Transformation|GetActorLocation))
  (bind _explosionforcescalar (Variables|Default|GetExplosionForceScalar))
  (bind _bodycolororigin (Variables|Default|GetBodyColorOrigin))
  (bind _returnvalue_3 (Math|Rotator|FindLookatRotation _returnvalue _returnvalue_2))
  (bind (_r _g _b _a) (Math|Color|BreakColor _bodycolororigin))
  (bind _returnvalue_4 (* 0.0 _explosionforcescalar))
  (bind _returnvalue_5 (Math|Vector|GetForwardVector _returnvalue_3))
  (bind _returnvalue_6 (* _returnvalue_5 _returnvalue_4))
  (bind _output_get (Variables|Default|SetbCharacterDead (<= (- (Variables|Default|GetHP) Damage) 0.0)))
  (if _output_get
    (Variables|Default|SetHP 0.0)
    (Utilities|FlowControl|Sequence
      (:then_0
        (Rendering|Material|SetVectorParameterValue (Variables|Default|GetDMIBody) "bodyColor" "(R=0.000000,G=0.000000,B=0.000000,A=1.000000)" :!class /Script/Engine.MaterialInstanceDynamic)
        (Physics|SetSimulatePhysics (Variables|Character|GetMesh) true)
        (Physics|SetSimulatePhysics (Variables|Default|GetGunMesh) true)
        (Input|DisableInput (Game|GetPlayerController 0)))
      (:then_1
        (if (Actor|ActorHasTag DamageCauser "Bomb")
          (Physics|AddForce (Variables|Character|GetMesh) _returnvalue_6 "None" false)
          (Physics|AddForce (Variables|Default|GetGunMesh) _returnvalue_6 "None" false))))
    (else
      (Variables|Default|SetHP (- (Variables|Default|GetHP) Damage))
      (bind _black (Timeline|ColorChange Play)
        (:Update
          (Rendering|Material|SetVectorParameterValue (Variables|Default|GetDMIBody) "bodyColor" (Utilities|Struct|MakeLinearColor (* _black _r) (* _black _g) (* _black _b) _a) :!class /Script/Engine.MaterialInstanceDynamic))))))

(event EventTick
  (params (DeltaSeconds :type Float%20%28single-precision%29))
  (bind _curammocount (Variables|Default|GetCurAmmoCount))
  (Utilities|FlowControl|Gate true
    (:Exit
      (if (Variables|Default|GetAimPressed)
        (Utilities|FlowControl|Delay 0.1)
        (CallFunction|Fire 10000 _curammocount)
        (if (> _curammocount 0)
          (Math|Integer|DecrementInt _curammocount
            (:%20%20
              (CallFunction|ShowAmmoCount))))))))

(event Input|ActionEvents|InputActionSprint
  (params (Key :type Key%20Structure :default "None"))
  (:Pressed
    (Variables|Default|SetSprintPressed true)
    (CallFunction|SetMaxSpeed :!label _label))
  (:Released
    (Variables|Default|SetSprintPressed false)
    (goto _label)))

(event Input|ActionEvents|InputActionWalk
  (params (Key :type Key%20Structure :default "None"))
  (:Pressed
    (Variables|Default|SetWalkPressed true)
    (CallFunction|SetMaxSpeed :!label _label))
  (:Released
    (Variables|Default|SetWalkPressed false)
    (goto _label)))

(event Input|ActionEvents|InputActionAim
  (params (Key :type Key%20Structure :default "None"))
  (bind _charactermovement (Variables|Character|GetCharacterMovement))
  (:Pressed
    (if (not (or (Variables|Default|GetSprintPressed) (Variables|Default|GetJumpPressed)))
      (Variables|Default|SetAimPressed true)
      (CallFunction|SetMaxSpeed)
      (Utilities|IsValid (Variables|Default|GetUMGAimRef)
        (:Is%20Valid
          _)
        (:Is%20Not%20Valid
          (bind _returnvalue (UserInterface|CreateWidget "/Game/MyContents/TPSGunner/UMG_TPSCharacter_Aim.UMG_TPSCharacter_Aim_C"))
          (bind _output_get (Variables|Default|SetUMGAimRef _returnvalue))))
      (UserInterface|Viewport|AddtoViewport _output_get 0)
      (Utilities|FlowControl|Sequence
        (:then_0
          ;[1 1 1] 자유로운 카메라 이동
          (Variables|/Script/Engine.CharacterMovementComponent|SetbUseControllerDesiredRotation _charactermovement false)
          (Variables|/Script/Engine.CharacterMovementComponent|SetbOrientRotationToMovement _charactermovement false)
          (Variables|Default|SetbUseControllerRotationYaw true))
        (:then_1
          (bind _fov (Timeline|ChangeFOV Play)
            (:Update
              (Camera|SetFieldOfView (Variables|Default|GetCamera) _fov)))))))
  (:Released
    (Variables|Default|SetAimPressed false)
    (CallFunction|SetMaxSpeed)
    (Utilities|IsValid (Variables|Default|GetUMGAimRef)
      (:Is%20Valid
        (Widget|RemovefromParent (Variables|Default|GetUMGAimRef))
        (Utilities|FlowControl|Sequence
          (:then_0
            ;[1 1 1] 카메라가 등만 보이게
            (Variables|/Script/Engine.CharacterMovementComponent|SetbUseControllerDesiredRotation _charactermovement true)
            (Variables|/Script/Engine.CharacterMovementComponent|SetbOrientRotationToMovement _charactermovement true)
            (Variables|Default|SetbUseControllerRotationYaw false))
          (:then_1
            (Timeline|ChangeFOV Reverse)))))))

(event Input|ActionEvents|InputActionFire
  (params (Key :type Key%20Structure :default "None"))
  (bind _curammocount (Variables|Default|GetCurAmmoCount))
  (:Pressed
    (Utilities|FlowControl|Gate true) ; enters at Open
  )
  (:Released
    (Utilities|FlowControl|Gate true) ; enters at Close
  ))

(event Input|ActionEvents|InputActionJump
  (params (Key :type Key%20Structure :default "None"))
  (:Pressed
    (if (not (or (Variables|Default|GetCrouchPressed) (Variables|Default|GetAimPressed)))
      (if (not (Variables|Default|GetJumpPressed))
        (Variables|Default|SetJumpPressed true)
        (Character|Jump))))
  (:Released
    (Character|StopJumping)))

(event Input|ActionEvents|InputActionCrouch
  (params (Key :type Key%20Structure :default "None"))
  (:Pressed
    (Variables|Default|SetCrouchPressed (not (Variables|Default|GetCrouchPressed)))
    (CallFunction|SetMaxSpeed)))

(event Input|ActionEvents|InputActionReload
  (params (Key :type Key%20Structure :default "None"))
  (bind _ammomagazinesize (Variables|Default|GetAmmoMagazineSize))
  (:Pressed
    (if (< (Variables|Default|GetCurAmmoCount) (Variables|Default|GetAmmoMagazineSize))
      (if (>= (Variables|Default|GetMaxAmmoCount) (Variables|Default|GetAmmoMagazineSize))
        (Variables|Default|SetMaxAmmoCount (- (+ (Variables|Default|GetMaxAmmoCount) (Variables|Default|GetCurAmmoCount)) _ammomagazinesize) :!label _label)
        (Variables|Default|SetCurAmmoCount _ammomagazinesize)
        (CallFunction|ShowAmmoCount)
        (Audio|PlaySound2D "/Game/UnrealFreeAssets/MilitaryWeapDark/Sound/Rifle/Wavs/Rifle_Reload01.Rifle_Reload01" 1.0 1.0 0.0 0 0)
        (Variables|Default|SetReloadPressed true)
        (elif (>= (+ (Variables|Default|GetCurAmmoCount) (Variables|Default|GetMaxAmmoCount)) (Variables|Default|GetAmmoMagazineSize))
          (goto _label)
          (elif (> (Variables|Default|GetMaxAmmoCount) 0)
            ;[1 1 1] Last One!
            (Variables|Default|SetCurAmmoCount (+ (Variables|Default|GetMaxAmmoCount) (Variables|Default|GetCurAmmoCount)))
            (Variables|Default|SetMaxAmmoCount 0)
            (CallFunction|ShowAmmoCount)))))))

(event Input|AxisEvents|InputAxisMoveForward
  (params (AxisValue :type Float%20%28single-precision%29))
  (Pawn|Input|AddMovementInput (Math|Vector|GetForwardVector (Math|Rotator|MakeRotator 0.0 0.0 (.Yaw (Math|Rotator|BreakRotator (Pawn|GetControlRotation :!class /Script/Engine.Pawn))))) AxisValue false))

(event Input|AxisEvents|InputAxisMoveRight
  (params (AxisValue :type Float%20%28single-precision%29))
  (Pawn|Input|AddMovementInput (Math|Vector|GetRightVector (Math|Rotator|MakeRotator 0.0 0.0 (.Yaw (Math|Rotator|BreakRotator (Pawn|GetControlRotation :!class /Script/Engine.Pawn))))) AxisValue false))

(event Input|AxisEvents|InputAxisTurn
  (params (AxisValue :type Float%20%28single-precision%29))
  (Pawn|Input|AddControllerYawInput AxisValue))

(event Input|AxisEvents|InputAxisLookup
  (params (AxisValue :type Float%20%28single-precision%29))
  (Pawn|Input|AddControllerPitchInput AxisValue))

(event Input|KeyboardEvents|2
  (params (Key :type Key%20Structure :default "None"))
  (bind _returnvalue (Game|GetPlayerController 0))
  (bind _montagepool (Variables|Default|GetMontagePool))
  (:Pressed
    (Input|DisableInput _returnvalue)
    (Animation|Montage|MontagePlay (Components|SkeletalMesh|GetAnimInstance (Variables|Character|GetMesh)) (Utilities|Array|Get(acopy) _montagepool (Math|Random|RandomIntegerinRange 0 (Utilities|Array|Length _montagepool))) 1.0 "MontageLength" 0.0 true)
    (Input|EnableInput _returnvalue)
    (Game|Damage|ApplyDamage self 1e+01 0 0)))

(fn ConstructionScript
  (bind _mesh (Variables|Character|GetMesh))
  (bind _returnvalue (Rendering|Material|CreateDynamicMaterialInstance _mesh 0 0 "None" :!class /Script/Engine.PrimitiveComponent))
  (bind _output_get (Variables|Default|SetDMIBody _returnvalue))
  (Rendering|Material|SetMaterial _mesh 0 _output_get)
  (bind _returnvalue_2 (Rendering|Material|GetVectorParameterValue _output_get "bodyColor" :!class /Script/Engine.MaterialInstanceDynamic))
  (Variables|Default|SetBodyColorOrigin _returnvalue_2))

(fn SetMaxSpeed
  (bind _charactermovement (Variables|Character|GetCharacterMovement))
  (if (Math|Boolean|ORBoolean (Variables|Default|GetCrouchPressed) (Variables|Default|GetWalkPressed) (Variables|Default|GetAimPressed))
    (Variables|/Script/Engine.CharacterMovementComponent|SetMaxWalkSpeed _charactermovement 2e+02)
    (elif (Variables|Default|GetSprintPressed)
      (Variables|/Script/Engine.CharacterMovementComponent|SetMaxWalkSpeed _charactermovement 1e+03)
      (else
        (Variables|/Script/Engine.CharacterMovementComponent|SetMaxWalkSpeed _charactermovement 6e+02)))))

(fn Fire
  (params (AttackRange :type Integer) (LeftAmmo :type Integer))
  (bind _camera (Variables|Default|GetCamera))
  (bind _returnvalue (Transformation|GetWorldLocation _camera))
  (if (> LeftAmmo 0)
    (Utilities|FlowControl|Sequence
      (:then_0
        (Animation|Montage|MontagePlay (Components|SkeletalMesh|GetAnimInstance (Variables|Character|GetMesh)) "/Game/MyContents/TPSGunner/AMT_Fire_Rifle_Ironsights_AnimMontage.AMT_Fire_Rifle_Ironsights_AnimMontage" 1.0 "MontageLength" 0.0 true))
      (:then_1
        (CameraShakes|StartCameraShake (Game|GetPlayerCameraManager 0) "/Game/MyContents/TPSGunner/BP_FireCamShake.BP_FireCamShake_C" 1.0 "CameraLocal" "0, 0, 0"))
      (:then_2
        (Effects|SpawnEmitteratLocation "/Game/UnrealFreeAssets/MilitaryWeapDark/FX/P_AssaultRifle_MuzzleFlash.P_AssaultRifle_MuzzleFlash" (Transformation|GetWorldLocation (Variables|Default|GetGunMuzzle))))
      (:then_3
        (Audio|PlaySound2D "/Game/UnrealFreeAssets/MilitaryWeapDark/Sound/Rifle/RifleB_Fire_Cue.RifleB_Fire_Cue" 1.0 1.0 0.0 0 0))
      (:then_4
        (bind (_outhit _returnvalue_2) (Collision|LineTraceByChannel _returnvalue (+ _returnvalue (* (Math|Vector|GetForwardVector (Pawn|GetControlRotation :!class /Script/Engine.Pawn)) AttackRange)) "TraceTypeQuery1" false 0 "None"))
        (if _returnvalue_2
          (Game|Damage|ApplyDamage (.HitActor (Collision|BreakHitResult _outhit)) 4e+01 0 0)
          (Effects|SpawnEmitteratLocation "/Game/UnrealFreeAssets/MilitaryWeapDark/FX/P_Impact_Metal_Medium_01.P_Impact_Metal_Medium_01" (+ (.ImpactPoint (Collision|BreakHitResult _outhit)) (* (.ImpactNormal (Collision|BreakHitResult _outhit)) 10)))))
      (:then_5
        (return)))
    (else
      (Audio|PlaySound2D "/Game/UnrealFreeAssets/MilitaryWeapDark/Sound/Rifle/Rifle_AmmoPickup_Cue.Rifle_AmmoPickup_Cue" 1.0 1.0 0.0 0 0))))

(fn ShowAmmoCount
  (Development|PrintString (Utilities|String|Append "Cur : " (Utilities|String|ToString(Integer) (Variables|Default|GetCurAmmoCount)) "Max : " (Utilities|String|ToString(Integer) (Variables|Default|GetMaxAmmoCount)))))