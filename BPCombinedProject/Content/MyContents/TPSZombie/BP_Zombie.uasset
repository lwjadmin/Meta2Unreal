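; BP_Zombie is a zombie enemy for a third-person shooter, with health, a contact attack and a ragdoll death.
; Incoming damage lowers HP, and at zero it sets IsDead, turns on mesh physics and disables capsule collision.
; Sphere overlap sets IsAttacking and deals one fixed hit to any overlapping actor, without checking IsDead, and end overlap clears the flag.
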(event OnComponentBeginOverlap(Sphere)
  (params (OverlappedComponent :type Primitive%20Component%20Object%20Reference) (OtherActor :type Actor%20Object%20Reference) (OtherComp :type Primitive%20Component%20Object%20Reference) (OtherBodyIndex :type Integer) (bFromSweep :type Boolean) (SweepResult :type Hit%20Result%20Structure%20%28by%20ref%29))
  (Development|PrintString "Attack!")
  (Variables|Default|SetIsAttacking true)
  (Game|Damage|ApplyDamage OtherActor 1e+01 0 0))

(event OnComponentEndOverlap(Sphere)
  (params (OverlappedComponent :type Primitive%20Component%20Object%20Reference) (OtherActor :type Actor%20Object%20Reference) (OtherComp :type Primitive%20Component%20Object%20Reference) (OtherBodyIndex :type Integer))
  (Development|PrintString "End Attack")
  (Variables|Default|SetIsAttacking false))

(event Game|Damage|EventAnyDamage
  (params (Damage :type Float%20%28single-precision%29) (DamageType :type Damage%20Type%20Object%20Reference) (InstigatedBy :type Controller%20Object%20Reference) (DamageCauser :type Actor%20Object%20Reference))
  (bind _output_get (Variables|Default|SetHP (- (Variables|Default|GetHP) Damage)))
  (if (and (not (Variables|Default|GetIsDead)) (<= _output_get 0.0))
    (Variables|Default|SetIsDead true)
    (Physics|SetSimulatePhysics (Variables|Character|GetMesh) true)
    (Collision|SetCollisionEnabled (Variables|Collision|GetCapsuleComponent) "NoCollision")))

(fn ConstructionScript)