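; Third-person shooter player character Blueprint handling camera-relative movement, jumping, aiming and firing.
; Crouch toggle and held sprint, walk and aim flags feed SetMaxSpeed to choose walk speed.
; Aiming shows a widget, switches to controller-yaw rotation and drives an FOV timeline, enabling fire effects: montage, camera shake, muzzle explosion and sound, without hit logic.
; Keys 1 and 2 trigger ragdoll with mesh detachment and random hit-react montages.
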(event EventBeginPlay
  (bind _montagepool (Variables|Default|GetMontagePool))
  (Utilities|Array|Add _montagepool "/Game/MyContents/Hit_React_2_Montage.Hit_React_2_Montage")
  (Utilities|Array|Add _montagepool "/Game/MyContents/Hit_React_3_Montage.Hit_React_3_Montage")
  (Utilities|Array|Add _montagepool "/Game/MyContents/Hit_React_4_Montage.Hit_React_4_Montage"))

(event Input|ActionEvents|InputActionSprint
  (params (Key :type Key%20Structure :default "None"))
  (:Pressed
    (Variables|Default|SetSprintPressed true)
    (CallFunction|SetMaxSpeed :!label _label))
  (:Released
    (Variables|Default|SetSprintPressed false)
    (goto _label)))

(event Input|ActionEvents|InputActionWalk
  (params (Key :type Key%20Structure :default "None"))
  (:Pressed
    (Variables|Default|SetWalkPressed true)
    (CallFunction|SetMaxSpeed :!label _label))
  (:Released
    (Variables|Default|SetWalkPressed false)
    (goto _label)))

(event Input|ActionEvents|InputActionAim
  (params (Key :type Key%20Structure :default "None"))
  (bind _charactermovement (Variables|Character|GetCharacterMovement))
  (:Pressed
    (if (not (or (Variables|Default|GetSprintPressed) (Variables|Default|GetJumpPressed)))
      (Variables|Default|SetAimPressed true)
      (CallFunction|SetMaxSpeed)
      (Utilities|IsValid (Variables|Default|GetUMGAimRef)
        (:Is%20Valid
          _)
        (:Is%20Not%20Valid
          (bind _returnvalue (UserInterface|CreateWidget "/Game/MyContents/UMG_TPSCharacter_Aim.UMG_TPSCharacter_Aim_C"))
          (bind _output_get (Variables|Default|SetUMGAimRef _returnvalue))))
      (UserInterface|Viewport|AddtoViewport _output_get 0)
      (Utilities|FlowControl|Sequence
        (:then_0
          (Variables|/Script/Engine.CharacterMovementComponent|SetbUseControllerDesiredRotation _charactermovement false)
          (Variables|/Script/Engine.CharacterMovementComponent|SetbOrientRotationToMovement _charactermovement false)
          (Variables|Default|SetbUseControllerRotationYaw true))
        (:then_1
          (bind _fov (Timeline|ChangeFOV Play)
            (:Update
              (Camera|SetFieldOfView (Variables|Default|GetCamera) _fov)))))))
  (:Released
    (Variables|Default|SetAimPressed false)
    (CallFunction|SetMaxSpeed)
    (Utilities|IsValid (Variables|Default|GetUMGAimRef)
      (:Is%20Valid
        (Widget|RemovefromParent (Variables|Default|GetUMGAimRef))
        (Utilities|FlowControl|Sequence
          (:then_0
            (Variables|/Script/Engine.CharacterMovementComponent|SetbUseControllerDesiredRotation _charactermovement true)
            (Variables|/Script/Engine.CharacterMovementComponent|SetbOrientRotationToMovement _charactermovement true)
            (Variables|Default|SetbUseControllerRotationYaw false))
          (:then_1
            (Timeline|ChangeFOV Reverse)))))))

(event Input|ActionEvents|InputActionFire
  (params (Key :type Key%20Structure :default "None"))
  (:Pressed
    (if (Variables|Default|GetAimPressed)
      (Animation|Montage|MontagePlay (Components|SkeletalMesh|GetAnimInstance (Variables|Character|GetMesh)) "/Game/MyContents/AMT_Fire_Rifle_Ironsights_AnimMontage.AMT_Fire_Rifle_Ironsights_AnimMontage" 1.0 "MontageLength" 0.0 true)
      (CameraShakes|StartCameraShake (Game|GetPlayerCameraManager 0) "/Game/MyContents/BP_FireCamShake.BP_FireCamShake_C" 1.0 "CameraLocal" "0, 0, 0")
      (Effects|SpawnEmitteratLocation "/Game/StarterContent/Particles/P_Explosion.P_Explosion" (Transformation|GetWorldLocation (Variables|Default|GetGunMuzzle)))
      (Audio|PlaySound2D "/Game/StarterContent/Audio/Explosion01.Explosion01" 1.0 1.0 0.0 0 0))))

(event Input|ActionEvents|InputActionJump
  (params (Key :type Key%20Structure :default "None"))
  (:Pressed
    (if (not (or (Variables|Default|GetCrouchPressed) (Variables|Default|GetAimPressed)))
      (if (not (Variables|Default|GetJumpPressed))
        (Variables|Default|SetJumpPressed true)
        (Character|Jump))))
  (:Released
    (Character|StopJumping)))

(event Input|ActionEvents|InputActionCrouch
  (params (Key :type Key%20Structure :default "None"))
  (:Pressed
    (Variables|Default|SetCrouchPressed (not (Variables|Default|GetCrouchPressed)))
    (CallFunction|SetMaxSpeed)))

(event Input|AxisEvents|InputAxisMoveForward
  (params (AxisValue :type Float%20%28single-precision%29))
  (Pawn|Input|AddMovementInput (Math|Vector|GetForwardVector (Math|Rotator|MakeRotator 0.0 0.0 (.Yaw (Math|Rotator|BreakRotator (Pawn|GetControlRotation :!class /Script/Engine.Pawn))))) AxisValue false))

(event Input|AxisEvents|InputAxisMoveRight
  (params (AxisValue :type Float%20%28single-precision%29))
  (Pawn|Input|AddMovementInput (Math|Vector|GetRightVector (Math|Rotator|MakeRotator 0.0 0.0 (.Yaw (Math|Rotator|BreakRotator (Pawn|GetControlRotation :!class /Script/Engine.Pawn))))) AxisValue false))

(event Input|AxisEvents|InputAxisTurn
  (params (AxisValue :type Float%20%28single-precision%29))
  (Pawn|Input|AddControllerYawInput AxisValue))

(event Input|AxisEvents|InputAxisLookup
  (params (AxisValue :type Float%20%28single-precision%29))
  (Pawn|Input|AddControllerPitchInput AxisValue))

(event Input|KeyboardEvents|1
  (params (Key :type Key%20Structure :default "None"))
  (bind _staticmesh (Variables|Default|GetStaticMesh))
  (:Pressed
    (Physics|SetSimulatePhysics (Variables|Character|GetMesh) true)
    (Physics|SetSimulatePhysics _staticmesh true)
    (Transformation|DetachFromComponent _staticmesh "KeepWorld" "KeepWorld" "KeepWorld" true)
    (Input|DisableInput (Game|GetPlayerController 0))))

(event Input|KeyboardEvents|2
  (params (Key :type Key%20Structure :default "None"))
  (bind _returnvalue (Game|GetPlayerController 0))
  (bind _montagepool (Variables|Default|GetMontagePool))
  (:Pressed
    (Input|DisableInput _returnvalue)
    (Animation|Montage|MontagePlay (Components|SkeletalMesh|GetAnimInstance (Variables|Character|GetMesh)) (Utilities|Array|Get(acopy) _montagepool (Math|Random|RandomIntegerinRange 0 (Utilities|Array|Length _montagepool))) 1.0 "MontageLength" 0.0 true)
    (Input|EnableInput _returnvalue)))

(fn ConstructionScript)

(fn SetMaxSpeed
  (bind _charactermovement (Variables|Character|GetCharacterMovement))
  (if (Math|Boolean|ORBoolean (Variables|Default|GetCrouchPressed) (Variables|Default|GetWalkPressed) (Variables|Default|GetAimPressed))
    (Variables|/Script/Engine.CharacterMovementComponent|SetMaxWalkSpeed _charactermovement 2e+02)
    (elif (Variables|Default|GetSprintPressed)
      (Variables|/Script/Engine.CharacterMovementComponent|SetMaxWalkSpeed _charactermovement 1e+03)
      (else
        (Variables|/Script/Engine.CharacterMovementComponent|SetMaxWalkSpeed _charactermovement 6e+02)))))