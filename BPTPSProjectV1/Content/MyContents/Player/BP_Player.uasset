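; Player character Blueprint handling movement, stamina, health, rifle ammo and the HUD widget.
; Tick drains or regenerates stamina and updates walk speed, which scales with stamina outside walking and sprinting; jumping also costs stamina.
; Damage triggers camera shake, a timeline-blended upper-body physics reaction and health-based body darkening via a dynamic material; death ragdolls the mesh and disables input.
; Reload refills the magazine from reserve ammo, and key 1 applies self-damage.
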(event EventBeginPlay
  (bind _returnvalue (UserInterface|CreateWidget "/Game/MyContents/UMG_PlayerUI.UMG_PlayerUI_C" (Game|GetPlayerController 0)))
  (bind _output_get (Variables|Default|SetRefGUIWidget _returnvalue))
  (UserInterface|Viewport|AddtoViewport _output_get 0))

(event Game|Damage|EventAnyDamage
  (params (Damage :type Float%20%28single-precision%29) (DamageType :type Damage%20Type%20Object%20Reference) (InstigatedBy :type Controller%20Object%20Reference) (DamageCauser :type Actor%20Object%20Reference))
  (bind _returnvalue (Utilities|Name|MakeLiteralName "spine_01"))
  (bind _meshbodycolororigin (Variables|Default|GetMeshBodyColorOrigin))
  (bind _mesh (Variables|Character|GetMesh))
  (bind (_r _g _b _a) (Utilities|Struct|BreakLinearColor _meshbodycolororigin))
  ;[1 1 1] Damaged & Die
  (if (not (Variables|Default|GetbIsDead))
    (bind _output_get (Variables|Default|SetbIsDead (<= (- (Variables|Default|GetCurHP) Damage) 0.0)))
    (if _output_get
      (Variables|Default|SetCurHP 0.0)
      (Utilities|FlowControl|Sequence
        (:then_0
          (bind _blend_weight (Timeline|ChangeBlendWeight Stop)
            (:Update
              (Class|SkeletalMeshComponent|SetAllBodiesBelowPhysicsBlendWeight _mesh _returnvalue _blend_weight false true))
            (:Finished
              (Class|SkeletalMeshComponent|SetAllBodiesBelowSimulatePhysics _mesh _returnvalue false true))))
        (:then_1
          (Class|SkeletalMeshComponent|SetAllBodiesBelowPhysicsBlendWeight _mesh _returnvalue 0.0 false true)
          (Input|DisableInput (Game|GetPlayerController 0))
          (Physics|SetSimulatePhysics (Variables|Character|GetMesh) true)
          (Collision|SetCollisionEnabled (Variables|Collision|GetCapsuleComponent) "NoCollision")
          (Pawn|Components|CharacterMovement|DisableMovement (Variables|Character|GetCharacterMovement))
          (Audio|PlaySound2D "/Game/MyContents/Player/Sound/CharacterDeathCue.CharacterDeathCue" 1.0 1.0 0.0 0 0))
        (:then_2
          (Rendering|Material|SetVectorParameterValue (Variables|Default|GetMI_Mesh) "BodyColor" (Variables|Default|GetMeshBodyColorDead) :!class /Script/Engine.MaterialInstanceDynamic)))
      (else
        (Variables|Default|SetCurHP (- (Variables|Default|GetCurHP) Damage))
        (Utilities|FlowControl|Sequence
          (:then_0
            (CameraShakes|StartCameraShake (Game|GetPlayerCameraManager 0) "/Game/MyContents/Player/BP_CameraShake.BP_CameraShake_C" 1.0 "CameraLocal" "0, 0, 0")
            (Audio|PlaySound2D "/Game/MyContents/Player/Sound/CharacterDamaged.CharacterDamaged" 1.0 1.0 0.0 0 0)
            (Class|SkeletalMeshComponent|SetAllBodiesBelowSimulatePhysics _mesh _returnvalue true true)
            (Timeline|ChangeBlendWeight PlayFromStart))
          (:then_1
            (Rendering|Material|SetVectorParameterValue (Variables|Default|GetMI_Mesh) "BodyColor" (Utilities|Struct|MakeLinearColor (* _r (/ (Variables|Default|GetCurHP) (Variables|Default|GetMaxHP))) (* _g (/ (Variables|Default|GetCurHP) (Variables|Default|GetMaxHP))) (* _b (/ (Variables|Default|GetCurHP) (Variables|Default|GetMaxHP))) (* _a (/ (Variables|Default|GetCurHP) (Variables|Default|GetMaxHP)))) :!class /Script/Engine.MaterialInstanceDynamic)))))))

(event EventTick
  (params (DeltaSeconds :type Float%20%28single-precision%29))
  (bind _maxstamina (Variables|Default|GetMaxStamina))
  ;[1 1 1] Run
  (if (Variables|Default|GetbIsSprinting)
    (Variables|Default|SetCurStamina (Math|Float|Clamp(Float) (- (Variables|Default|GetCurStamina) (* DeltaSeconds 2e+01)) 0.0 _maxstamina))
    (else
      (Variables|Default|SetCurStamina (Math|Float|Clamp(Float) (+ (Variables|Default|GetCurStamina) (* DeltaSeconds 1e+01)) 0.0 _maxstamina))))
  (CallFunction|SetCharacterWalkSpeed))

(event Input|ActionEvents|InputActionJump
  (params (Key :type Key%20Structure :default "None"))
  ;[1 1 1] WASD, Jump
  (:Pressed
    (if (not (Variables|Default|GetbIsJumping))
      (Variables|Default|SetCurStamina (* (Variables|Default|GetCurStamina) 0.9))
      (Character|Jump)
      (Variables|Default|SetbIsJumping true)))
  (:Released
    (Character|StopJumping)))

(event Input|AxisEvents|InputAxisLookUp
  (params (AxisValue :type Float%20%28single-precision%29))
  ;[1 1 1] WASD, Jump
  (Pawn|Input|AddControllerPitchInput AxisValue))

(event Input|AxisEvents|InputAxisTurn
  (params (AxisValue :type Float%20%28single-precision%29))
  ;[1 1 1] WASD, Jump
  (Pawn|Input|AddControllerYawInput AxisValue))

(event Input|AxisEvents|InputAxisMoveForward
  (params (AxisValue :type Float%20%28single-precision%29))
  ;[1 1 1] WASD, Jump
  (Pawn|Input|AddMovementInput (Math|Vector|GetForwardVector (Math|Rotator|MakeRotator 0.0 0.0 (.Yaw (Math|Rotator|BreakRotator (Pawn|GetControlRotation :!class /Script/Engine.Pawn))))) AxisValue false))

(event Input|AxisEvents|InputAxisMoveRight
  (params (AxisValue :type Float%20%28single-precision%29))
  ;[1 1 1] WASD, Jump
  (Pawn|Input|AddMovementInput (Math|Vector|GetRightVector (Math|Rotator|MakeRotator 0.0 0.0 (.Yaw (Math|Rotator|BreakRotator (Pawn|GetControlRotation :!class /Script/Engine.Pawn))))) AxisValue false))

(event Input|KeyboardEvents|1
  (params (Key :type Key%20Structure :default "None"))
  ;[1 1 1] Damaged & Die
  (:Pressed
    (Game|Damage|ApplyDamage self 1e+01 0 0)))

(event Input|KeyboardEvents|LeftShift
  (params (Key :type Key%20Structure :default "None"))
  ;[1 1 1] Run
  (:Pressed
    (if (> (/ (Variables|Default|GetCurStamina) (Variables|Default|GetMaxStamina)) 0.3)
      (Variables|Default|SetbIsSprinting true)
      (CallFunction|SetCharacterWalkSpeed :!label _label)))
  (:Released
    (Variables|Default|SetbIsSprinting false)
    (goto _label)))

(event Input|KeyboardEvents|LeftCtrl
  (params (Key :type Key%20Structure :default "None"))
  ;[1 1 1] Run
  (:Pressed
    (Variables|Default|SetbIsWalking true)
    (CallFunction|SetCharacterWalkSpeed :!label _label))
  (:Released
    (Variables|Default|SetbIsWalking false)
    (goto _label)))

(event Input|KeyboardEvents|R
  (params (Key :type Key%20Structure :default "None"))
  (:Pressed
    (CallFunction|Reload)))

(fn ConstructionScript
  (bind _returnvalue (Rendering|Material|CreateDynamicMaterialInstance (Variables|Character|GetMesh) 0 0 "BodyColor" :!class /Script/Engine.PrimitiveComponent))
  (bind _output_get (Variables|Default|SetMI_Mesh _returnvalue))
  (bind _returnvalue_2 (Rendering|Material|GetVectorParameterValue _output_get "BodyColor" :!class /Script/Engine.MaterialInstanceDynamic))
  (Variables|Default|SetMeshBodyColorOrigin _returnvalue_2))

(fn SetCharacterWalkSpeed
  (bind _charactermovement (Variables|Character|GetCharacterMovement))
  (if (Variables|Default|GetbIsWalking)
    (Variables|Default|SetbIsSprinting false)
    (Variables|/Script/Engine.CharacterMovementComponent|SetMaxWalkSpeed _charactermovement 2e+02)
    (elif (Variables|Default|GetbIsSprinting)
      (if (> (Variables|Default|GetCurStamina) 0.0)
        (Variables|/Script/Engine.CharacterMovementComponent|SetMaxWalkSpeed _charactermovement 1.2e+03)
        (else
          (Variables|Default|SetbIsSprinting false)))
      (else
        (Variables|/Script/Engine.CharacterMovementComponent|SetMaxWalkSpeed _charactermovement (* (/ (Variables|Default|GetCurStamina) (Variables|Default|GetMaxStamina)) 6e+02))))))

(fn GetAmmunition
  (params (AmmoCount :type Integer))
  (Variables|Default|SetMaxAmmoCount (+ AmmoCount (Variables|Default|GetMaxAmmoCount)))
  (Audio|PlaySound2D "/Game/MilitaryWeapSilver/Sound/Rifle/Cues/Rifle_Reload_Cue.Rifle_Reload_Cue" 1.0 1.0 0.0 0 0))

(fn Reload
  (bind _ammomagazinesize (Variables|Default|GetAmmoMagazineSize))
  (if (< (Variables|Default|GetCurAmmoCount) (Variables|Default|GetAmmoMagazineSize))
    (if (>= (Variables|Default|GetMaxAmmoCount) (Variables|Default|GetAmmoMagazineSize))
      (Variables|Default|SetMaxAmmoCount (- (+ (Variables|Default|GetMaxAmmoCount) (Variables|Default|GetCurAmmoCount)) _ammomagazinesize) :!label _label)
      (Variables|Default|SetCurAmmoCount _ammomagazinesize)
      (Audio|PlaySound2D "/Game/MilitaryWeapSilver/Sound/Rifle/Cues/Rifle_Reload_Cue.Rifle_Reload_Cue" 1.0 1.0 0.0 0 0)
      (Variables|Default|SetbIsReloading true)
      (elif (>= (+ (Variables|Default|GetCurAmmoCount) (Variables|Default|GetMaxAmmoCount)) (Variables|Default|GetAmmoMagazineSize))
        (goto _label)
        (elif (> (Variables|Default|GetMaxAmmoCount) 0)
          (Variables|Default|SetCurAmmoCount (+ (Variables|Default|GetMaxAmmoCount) (Variables|Default|GetCurAmmoCount)))
          (Variables|Default|SetMaxAmmoCount 0))))))